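; Enemy assistant AI character that shoots at the player with a squirt gun and dances once the player dies.
; Wake-up damage or ForceAttackPlayer starts self-repeating, delay-driven rotation and montage attack loops, with a notify spawning each shot.
; Point damage either launches and stuns it, then resumes a floor-traced AIMoveTo chase, or drains health, causing random flinches and a ragdoll death.
; Attacks and stuns lock movement by zeroing walk speed.
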(event `RotateTowardsPlayer`
  (bind (_returnvalue_roll _returnvalue_pitch _returnvalue_yaw) (`KismetMathLibrary.BreakRotator` (`KismetMathLibrary.Conv_VectorToRotator` (`KismetMathLibrary.GetDirectionUnitVector` (`self.K2_GetActorLocation`) (`self.K2_GetActorLocation` (`GameplayStatics.GetPlayerCharacter` 0))))))
  (`self.K2_SetActorRotation` (`KismetMathLibrary.MakeRotator` 0.0 0.0 _returnvalue_yaw))
  (`KismetSystemLibrary.Delay` 0.01)
  (`self.RotateTowardsPlayer`))

(event `self.ReceiveBeginPlay`
  (set `self.Max Walk Speed` (`CharacterMovementComponent.MaxWalkSpeed` (`self.CharacterMovement`))))

(event `ForceAttackPlayer`
  (`self.RotateTowardsPlayer` :!label _label)
  (`self.AttackPlayer`))

(event `self.ReceiveAnyDamage`
  (params (Damage :type "Float (single-precision)") (DamageType :type "DamageType Object Reference") (InstigatedBy :type "Controller Object Reference") (DamageCauser :type "Actor Object Reference"))
  (if (== (`GameplayStatics.GetObjectClass` DamageType) "/Game/Blueprints/Damage/WakeUpEnemyAI_DamageType.WakeUpEnemyAI_DamageType_C")
    (goto _label)))

(event `ChasePlayer`
  (bind _returnvalue (`self.K2_GetActorLocation` (`GameplayStatics.GetPlayerCharacter` 0)))
  (if (not (or (`self.Dead`) (`self.Stunned`)))
    (bind (_outhit _returnvalue_2) (`KismetSystemLibrary.SphereTraceSingle` _returnvalue (- _returnvalue (0.0 0.0 5000.0)) 35.0 "TraceTypeQuery1"))
    (if _returnvalue_2
      (set `self.PlayerLocation` (`.Location` (`GameplayStatics.BreakHitResult` _outhit)))
      (else
        (set `self.PlayerLocation` _returnvalue)))
    (`|AIMoveTo` self (`self.PlayerLocation`) null
      (:`then`
        _)
      (:`OnSuccess`
        _)
      (:`OnFail`
        _))
    (`KismetSystemLibrary.Delay` 0.01)
    (`self.ChasePlayer`)))

(event `CannotMove`
  (set `self.CantMove` true)
  (set `CharacterMovementComponent.MaxWalkSpeed` 0.0 (`self.CharacterMovement`) :!label _label_2)
  (`KismetSystemLibrary.Delay` 0.01)
  (if (`self.CantMove`)
    (goto _label_2)))

(event `CanMoveAgain`
  (bind _charactermovement (`self.CharacterMovement`))
  (`KismetSystemLibrary.Delay` 0.01)
  (`KismetSystemLibrary.DelayUntilNextTick`)
  (`KismetSystemLibrary.DelayUntilNextTick`)
  (set `self.CantMove` false)
  (set `CharacterMovementComponent.MaxWalkSpeed` (`self.Max Walk Speed`) _charactermovement)
  (set `CharacterMovementComponent.GroundFriction` 0.0 _charactermovement))

(event `AttackPlayer`
  (bind _returnvalue (`SceneComponent.K2_GetComponentLocation` (`self.GunMesh`)))
  (bind _asbp_third_person_character (cast `/Game/Blueprints/BP_ThirdPersonCharacter` (`GameplayStatics.GetPlayerCharacter` 0)))
  (if (`/Game/Blueprints/BP_ThirdPersonCharacter.PlayerDead` _asbp_third_person_character)
    (`|PlayMontage` (`self.Mesh`) "/Game/Animations/Assistant/Twist_Dance__1__mixamo_com_Montage.Twist_Dance__1__mixamo_com_Montage" :!label _label_3
      (:`OnCompleted`
        (`|ExecutionSequence`
          (:`then_0`
            (goto _label_3)))))
    (elif (not (or (`self.Attacking`) (`self.Stunned`)))
      (set `self.Attacking` true)
      (`self.CannotMove`)
      (set `self.AttackMontageToPlay` "/Game/Animations/Assistant/FireGunAndReload.FireGunAndReload")
      (`GameplayStatics.PlaySoundAtLocation` "/Game/SFX/AssistantEffort1_Cue.AssistantEffort1_Cue" (`self.K2_GetActorLocation`) (struct) 1.0 1.0 0.0 null null null null)
      (`|PlayMontage` (`self.Mesh`) (`self.AttackMontageToPlay`)
        (:`OnBlendOut`
          (set `self.Attacking` false)
          (`KismetSystemLibrary.DelayUntilNextTick`)
          (`self.CanMoveAgain`)
          (`KismetSystemLibrary.Delay` (+ (`self.DelayUntilNextAttack`) (`KismetMathLibrary.RandomFloatInRange` -1.0 0.5)))
          (`KismetSystemLibrary.DelayUntilNextTick`)
          (`self.AttackPlayer`))
        (:`OnInterrupted`
          (set `self.Attacking` false))
        (:`OnNotifyBegin`
          (`|SpawnActorFromClass` "/Game/Blueprints/Projectiles/EnemySquirtGun_BP.EnemySquirtGun_BP_C" (`KismetMathLibrary.MakeTransform` _returnvalue (`KismetMathLibrary.Conv_VectorToRotator` (`KismetMathLibrary.GetDirectionUnitVector` _returnvalue (`self.K2_GetActorLocation` (`GameplayStatics.GetPlayerCharacter` 0))))) "Undefined" "MultiplyWithRoot" null null)
          (`ActorComponent.Activate` (`self.P_SquirtGun`) true)
          (`GameplayStatics.PlaySoundAtLocation` "/Game/SFX/AssistantShoot1_Cue.AssistantShoot1_Cue" (`self.K2_GetActorLocation`) (struct) 1.0 1.0 0.0 null null null null)
          (bind (_direction _newtrack_0) (`Timeline|Timeline` :!via `PlayFromStart`)
            (:`Update`
              (`SceneComponent.SetRelativeScale3D` (`self.GunMesh`) (`KismetMathLibrary.VLerp` (1.0 1.0 1.0) (0.6 0.3 0.3) _newtrack_0)))))))))

(event `self.ReceivePointDamage`
  (params (Damage :type "Float (single-precision)") (DamageType :type "DamageType Object Reference") (HitLocation :type "Vector Structure") (HitNormal :type "Vector Structure") (HitComponent :type "PrimitiveComponent Object Reference") (BoneName :type Name) (ShotFromDirection :type "Vector Structure") (InstigatedBy :type "Controller Object Reference") (DamageCauser :type "Actor Object Reference") (HitInfo :type "HitResult Structure (by ref)"))
  (bind _mesh (`self.Mesh`))
  (bind _charactermovement (`self.CharacterMovement`))
  (`|ExecutionSequence`
    (:`then_0`
      (if (== (`GameplayStatics.GetObjectClass` DamageType) "/Game/Blueprints/Damage/KnockBack_DamageType.KnockBack_DamageType_C")
        (`self.CannotMove`)
        (set `self.Stunned` true)
        (`KismetSystemLibrary.DelayUntilNextTick`)
        (set `CharacterMovementComponent.GroundFriction` 0.0 (`self.CharacterMovement`))
        (`self.LaunchCharacter` (* ShotFromDirection Damage 20000.0) true)
        (`|PlayMontage` (`self.Mesh`) "/Game/Animations/Assistant/Stunned__1__mixamo_com_Montage.Stunned__1__mixamo_com_Montage"
          (:`OnBlendOut`
            (`|PlayMontage` (`self.Mesh`) "/Game/Animations/Assistant/Getting_Up__9__mixamo_com_Montage.Getting_Up__9__mixamo_com_Montage"
              (:`OnBlendOut`
                (`self.CanMoveAgain`))
              (:`OnInterrupted`
                _)))
          (:`OnInterrupted`
            _))
        (set `self.Stunned` false)
        (`self.ChasePlayer`)
        (else
          (set `self.Health` (+ (* Damage -1.0) (`self.Health`)))
          (`GameplayStatics.PlaySoundAtLocation` "/Game/SFX/AssistantHurt1_Cue.AssistantHurt1_Cue" (`self.K2_GetActorLocation`) (struct) 1.0 1.0 0.0 null null null null)
          (`|ExecutionSequence`
            (:`then_0`
              (if (<= (`self.Health`) 0.0)
                (`|ExecutionSequence`
                  (:`then_0`
                    (`/Engine/EditorBlueprintResources/StandardMacros.DoOnce` false
                      (:`Completed`
                        (set `self.Dead` true)
                        (`PrimitiveComponent.SetCollisionEnabled` _mesh "QueryAndPhysics")
                        (`PrimitiveComponent.SetSimulatePhysics` _mesh true)
                        (`PrimitiveComponent.AddRadialImpulse` (`self.Mesh`) HitLocation 3000.0 3000.0 "RIF_Constant" true)
                        (set `SkeletalMeshComponent.bPauseAnims` true (`self.Mesh`))
                        (`PrimitiveComponent.SetCollisionEnabled` (`self.CapsuleComponent`) "NoCollision")
                        (set `CharacterMovementComponent.GravityScale` 0.0 _charactermovement)
                        (`PrimitiveComponent.SetEnableGravity` (`self.CapsuleComponent`) false)
                        (`CharacterMovementComponent.SetMovementMode` _charactermovement "MOVE_Flying" 0))))
                  (:`then_1`
                    (`PrimitiveComponent.AddRadialImpulse` (`self.Mesh`) HitLocation 3000.0 3000.0 "RIF_Constant" true)))
                (else
                  (`self.Flinch`))))
            (:`then_1`
              (bind _asbp_third_person_character (cast `/Game/Blueprints/BP_ThirdPersonCharacter` (`GameplayStatics.GetPlayerCharacter` 0)))
              (bind _hudwidget (`/Game/Blueprints/BP_ThirdPersonCharacter.HUDWidget` _asbp_third_person_character))
              (`UserWidget.PlayAnimation` _hudwidget (`/Game/UI/HUD_WBP.HitAnimTargetDot` _hudwidget) 0.0 1 "Forward" 1.0 false))))))))

(event `Flinch`
  (set `self.Stunned` true)
  (`self.CannotMove`)
  (switch `int` (`KismetMathLibrary.RandomIntegerInRange` 0 3)
    (:`Default`
      (set `self.HitReactToPlay` "/Game/Animations/Assistant/Hit_Reaction__15__mixamo_com_Montage.Hit_Reaction__15__mixamo_com_Montage" :!label _label_4))
    (:`0`
      (goto _label_4))
    (:`1`
      (set `self.HitReactToPlay` "/Game/Animations/Assistant/Hit_Reaction__16__mixamo_com_Montage.Hit_Reaction__16__mixamo_com_Montage"))
    (:`2`
      (set `self.HitReactToPlay` "/Game/Animations/Assistant/Hit_Reaction__17__mixamo_com_Montage.Hit_Reaction__17__mixamo_com_Montage"))
    (:`3`
      (set `self.HitReactToPlay` "/Game/Animations/Assistant/Standing_React_Large_Gut__3__mixamo_com_Montage.Standing_React_Large_Gut__3__mixamo_com_Montage")))
  (`|PlayMontage` (`self.Mesh`) (`self.HitReactToPlay`)
    (:`OnBlendOut`
      (set `self.Stunned` false)
      (`self.CanMoveAgain`))))

(fn `UserConstructionScript`)