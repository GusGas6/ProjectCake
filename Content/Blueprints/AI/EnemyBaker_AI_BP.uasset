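; Enemy baker melee AI, with a flag for a larger hammer-wielding Dark Chef that can be a mini-boss with music and HUD health bar.
; A wake-up damage type starts a looping chase toward the ground below the player; a detection capsule triggers random attack montages whose notifies toggle hit collision.
; Point damage drives flinches, knockback stuns and ragdoll death.
; At half health, the Dark Chef enrages, gaining speed and lightning AoE casts.
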(event `self.ReceiveBeginPlay`
  (bind _mesh (`self.Mesh`))
  (bind _chefhat (`self.ChefHat`))
  (bind _charactermovement (`self.CharacterMovement`))
  (if (`self.DarkChef`)
    (set `self.Max Walk Speed` 150.0)
    (set `CharacterMovementComponent.MaxWalkSpeed` 150.0 _charactermovement)
    (`PrimitiveComponent.SetMaterial` _mesh 0 "/Engine/MapTemplates/Sky/M_BlackBackground.M_BlackBackground")
    (`PrimitiveComponent.SetMaterial` _mesh 3 "/Game/Materials/RedRobe_Mat.RedRobe_Mat")
    (`PrimitiveComponent.SetMaterial` _chefhat 0 "/Engine/MapTemplates/Sky/M_BlackBackground.M_BlackBackground")
    (`SceneComponent.K2_SetRelativeLocation` _chefhat (0.0 0.0 35.0) false false)
    (`SceneComponent.SetRelativeScale3D` _chefhat (2.0 2.0 2.0))
    (`SceneComponent.SetHiddenInGame` (`self.Greathammer`) false false)
    (`SceneComponent.SetHiddenInGame` (`self.1hWeapon`) true false)
    (set `self.Base Damage` 5.0)
    (`self.SetActorScale3D` (1.6 1.6 1.6))
    (set `self.Health` (`self.DarkChefHealth`))
    (if (`self.MiniBoss`)
      (bind _asbp_third_person_character (cast `/Game/Blueprints/BP_ThirdPersonCharacter` (`GameplayStatics.GetPlayerCharacter` 0)))
      (bind _asmusic_controller_bp (cast `/Game/Blueprints/MusicController_BP` (`ChildActorComponent.ChildActor` (`/Game/Blueprints/BP_ThirdPersonCharacter.MusicController` _asbp_third_person_character))))
      (`/Game/Blueprints/MusicController_BP.Tier1BossMusic` _asmusic_controller_bp))
    (else
      (set `self.Max Walk Speed` (`CharacterMovementComponent.MaxWalkSpeed` _charactermovement)))))

(event `self.ReceiveAnyDamage`
  (params (Damage :type "Float (single-precision)") (DamageType :type "DamageType Object Reference") (InstigatedBy :type "Controller Object Reference") (DamageCauser :type "Actor Object Reference"))
  (if (== (`GameplayStatics.GetObjectClass` DamageType) "/Game/Blueprints/Damage/WakeUpEnemyAI_DamageType.WakeUpEnemyAI_DamageType_C")
    (`self.ChasePlayer`)
    (`/Engine/EditorBlueprintResources/StandardMacros.DoOnce` false
      (:`Completed`
        (if (`self.MiniBoss`)
          (bind _asbp_third_person_character (cast `/Game/Blueprints/BP_ThirdPersonCharacter` (`GameplayStatics.GetPlayerCharacter` 0)))
          (bind _hudwidget (`/Game/Blueprints/BP_ThirdPersonCharacter.HUDWidget` _asbp_third_person_character))
          (set `/Game/UI/HUD_WBP.CurrentBoss` self _hudwidget)
          (`UserWidget.PlayAnimation` _hudwidget (`/Game/UI/HUD_WBP.BossHealthbarFadeIn` _hudwidget) 0.0 1 "Forward" 1.0 false))))))

(event `ChasePlayer`
  (bind _returnvalue (`self.K2_GetActorLocation` (`GameplayStatics.GetPlayerCharacter` 0)))
  (if (not (or (`self.Dead`) (`self.Stunned`)))
    (bind (_outhit _returnvalue_2) (`KismetSystemLibrary.SphereTraceSingle` _returnvalue (- _returnvalue (0.0 0.0 5000.0)) 35.0 "TraceTypeQuery1"))
    (if _returnvalue_2
      (set `self.PlayerLocation` (`.Location` (`GameplayStatics.BreakHitResult` _outhit)))
      (else
        (set `self.PlayerLocation` _returnvalue)))
    (if (`PrimitiveComponent.IsOverlappingActor` (`self.PlayerDetectionCapsule`) (`GameplayStatics.GetPlayerCharacter` 0))
      (set `self.OverlappingPlayer` true)
      (`self.AttackPlayer`))
    (`|AIMoveTo` self (`self.PlayerLocation`) null
      (:`then`
        _)
      (:`OnSuccess`
        _)
      (:`OnFail`
        _))
    (`KismetSystemLibrary.Delay` 0.01)
    (`self.ChasePlayer`)))

(event `CannotMove`
  (set `self.CantMove` true)
  (set `CharacterMovementComponent.MaxWalkSpeed` 0.0 (`self.CharacterMovement`) :!label _label)
  (`KismetSystemLibrary.Delay` 0.01)
  (if (`self.CantMove`)
    (goto _label)))

(event `CanMoveAgain`
  (bind _charactermovement (`self.CharacterMovement`))
  (`KismetSystemLibrary.Delay` 0.01)
  (`KismetSystemLibrary.DelayUntilNextTick`)
  (`KismetSystemLibrary.DelayUntilNextTick`)
  (set `self.CantMove` false)
  (set `CharacterMovementComponent.MaxWalkSpeed` (`self.Max Walk Speed`) _charactermovement)
  (set `CharacterMovementComponent.GroundFriction` 0.0 _charactermovement))

(event `self.PlayerDetectionCapsule.OnComponentBeginOverlap`
  (params (OverlappedComponent :type "PrimitiveComponent Object Reference") (OtherActor :type "Actor Object Reference") (OtherComp :type "PrimitiveComponent Object Reference") (OtherBodyIndex :type Integer) (bFromSweep :type Boolean) (SweepResult :type "HitResult Structure (by ref)"))
  (cast `/Game/Blueprints/BP_ThirdPersonCharacter` OtherActor)
  (set `self.OverlappingPlayer` true)
  (`self.AttackPlayer`))

(event `self.PlayerDetectionCapsule.OnComponentEndOverlap`
  (params (OverlappedComponent :type "PrimitiveComponent Object Reference") (OtherActor :type "Actor Object Reference") (OtherComp :type "PrimitiveComponent Object Reference") (OtherBodyIndex :type Integer))
  (cast `/Game/Blueprints/BP_ThirdPersonCharacter` OtherActor)
  (set `self.OverlappingPlayer` false))

(event `AttackPlayer`
  (bind _returnvalue (`self.K2_GetActorLocation`))
  (bind _returnvalue_2 (`SceneComponent.K2_GetComponentLocation` (`self.LightningSpawnLocation`)))
  (bind _asbp_third_person_character (cast `/Game/Blueprints/BP_ThirdPersonCharacter` (`GameplayStatics.GetPlayerCharacter` 0)))
  (if (`/Game/Blueprints/BP_ThirdPersonCharacter.PlayerDead` _asbp_third_person_character)
    (`|PlayMontage` (`self.Mesh`) "/Game/Animations/Baker/Swing_Dancing_mixamo_com_Montage.Swing_Dancing_mixamo_com_Montage" :!label _label_2
      (:`OnCompleted`
        (`|ExecutionSequence`
          (:`then_0`
            (goto _label_2)))))
    (elif (not (or (`self.Attacking`) (`self.Stunned`)))
      (set `self.Attacking` true)
      (`self.CannotMove`)
      (if (`self.DarkChef`)
        (switch `int` (`KismetMathLibrary.RandomIntegerInRange` 0 3)
          (:`Default`
            (set `self.AttackMontageToPlay` "/Game/Animations/Baker/DarkChef/Great_Sword_Casting__7__mixamo_com_Montage.Great_Sword_Casting__7__mixamo_com_Montage" :!label _label_3))
          (:`0`
            (switch `int` (`KismetMathLibrary.RandomIntegerInRange` 0 2) :!label _label_4
              (:`Default`
                (set `self.AttackMontageToPlay` "/Game/Animations/Baker/Standing_Melee_Attack_Downward__5__mixamo_com_Montage.Standing_Melee_Attack_Downward__5__mixamo_com_Montage" :!label _label_5))
              (:`0`
                (goto _label_5))
              (:`1`
                (set `self.AttackMontageToPlay` "/Game/Animations/Baker/Standing_Melee_Combo_Attack_Ver__3__2__mixamo_com_Montage.Standing_Melee_Combo_Attack_Ver__3__2__mixamo_com_Montage"))
              (:`2`
                (set `self.AttackMontageToPlay` "/Game/Animations/Baker/Standing_Melee_Attack_360_High__7__mixamo_com_Montage.Standing_Melee_Attack_360_High__7__mixamo_com_Montage"))))
          (:`1`
            (goto _label_3))
          (:`2`
            (set `self.AttackMontageToPlay` "/Game/Animations/Baker/DarkChef/Heavy_Weapon_Swing__13__mixamo_com_Montage.Heavy_Weapon_Swing__13__mixamo_com_Montage"))
          (:`3`
            (set `self.AttackMontageToPlay` "/Game/Animations/Baker/DarkChef/Heavy_Weapon_Swing__14__mixamo_com_Montage.Heavy_Weapon_Swing__14__mixamo_com_Montage")))
        (else
          (goto _label_4)))
      (bind _notifyname (`|PlayMontage` (`self.Mesh`) (`self.AttackMontageToPlay`))
        (:`then`
          (if (`self.DarkChef`)
            (`GameplayStatics.PlaySoundAtLocation` "/Game/SFX/BakerAttack5_Cue.BakerAttack5_Cue" _returnvalue (struct) 1.0 1.0 0.0 null null null null)
            (else
              (`GameplayStatics.PlaySoundAtLocation` "/Game/SFX/DarkChefEffort4_Cue.DarkChefEffort4_Cue" _returnvalue (struct) 1.0 1.0 0.0 null null null null))))
        (:`OnBlendOut`
          (set `self.Attacking` false)
          (if (`self.OverlappingPlayer`)
            (`KismetSystemLibrary.DelayUntilNextTick`)
            (`self.AttackPlayer`)
            (else
              (`KismetSystemLibrary.DelayUntilNextTick`)
              (`self.CanMoveAgain`)
              (`self.ChasePlayer`))))
        (:`OnInterrupted`
          (`|ExecutionSequence`
            (:`then_0`
              (set `self.Attacking` false))
            (:`then_1`
              (`self.TurnOffAttackCollision` :!label _label_6))))
        (:`OnNotifyBegin`
          (`self.TurnOnAttackCollision`)
          (if (and (== _notifyname "Cast") (== (`self.AttackMontageToPlay`) "/Game/Animations/Baker/DarkChef/Great_Sword_Casting__7__mixamo_com_Montage.Great_Sword_Casting__7__mixamo_com_Montage"))
            (if (`self.Raging`)
              (`NiagaraFunctionLibrary.SpawnSystemAtLocation` "/Game/Vefects/Zap_VFX/VFX/Zap/Particles/NS_Zap_Red.NS_Zap_Red" _returnvalue_2 (struct) (3.0 3.0 3.0))
              (`|SpawnActorFromClass` "/Game/Blueprints/Damage/Aoe_Damage_BP.Aoe_Damage_BP_C" (`KismetMathLibrary.MakeTransform` _returnvalue_2) "Undefined" "MultiplyWithRoot" null 5.0 null 200.0 false 2000.0 2000.0 false null)
              (`GameplayStatics.PlaySoundAtLocation` "/Game/SFX/HeavyGroundImpact_Cue.HeavyGroundImpact_Cue" (`self.K2_GetActorLocation`) (struct) 1.0 1.0 0.0 null null null null)
              (`GameplayStatics.PlaySoundAtLocation` "/Game/SFX/LightningStrike1_Cue.LightningStrike1_Cue" (`self.K2_GetActorLocation`) (struct) 1.0 1.0 0.0 null null null null))))
        (:`OnNotifyEnd`
          (goto _label_6))))))

(event `self.Capsule.OnComponentBeginOverlap`
  (params (OverlappedComponent :type "PrimitiveComponent Object Reference") (OtherActor :type "Actor Object Reference") (OtherComp :type "PrimitiveComponent Object Reference") (OtherBodyIndex :type Integer) (bFromSweep :type Boolean) (SweepResult :type "HitResult Structure (by ref)"))
  (bind _asbp_third_person_character (cast `/Game/Blueprints/BP_ThirdPersonCharacter` OtherActor))
  (if (`/Game/Blueprints/BP_ThirdPersonCharacter.PlayerDead` _asbp_third_person_character)
    (goto _label_2)
    (else
      (`GameplayStatics.ApplyPointDamage` _asbp_third_person_character (`self.Base Damage`) (`KismetMathLibrary.GetDirectionUnitVector` (`self.K2_GetActorLocation`) (`self.K2_GetActorLocation` _asbp_third_person_character)) SweepResult null self))))

(event `self.Capsule1.OnComponentBeginOverlap`
  (params (OverlappedComponent :type "PrimitiveComponent Object Reference") (OtherActor :type "Actor Object Reference") (OtherComp :type "PrimitiveComponent Object Reference") (OtherBodyIndex :type Integer) (bFromSweep :type Boolean) (SweepResult :type "HitResult Structure (by ref)"))
  (bind _asbp_third_person_character (cast `/Game/Blueprints/BP_ThirdPersonCharacter` OtherActor))
  (if (`/Game/Blueprints/BP_ThirdPersonCharacter.PlayerDead` _asbp_third_person_character)
    (goto _label_2)
    (else
      (`GameplayStatics.ApplyPointDamage` _asbp_third_person_character (`self.Base Damage`) (`KismetMathLibrary.GetDirectionUnitVector` (`self.K2_GetActorLocation`) (`self.K2_GetActorLocation` _asbp_third_person_character)) SweepResult null self))))

(event `TurnOnAttackCollision`
  (if (`self.DarkChef`)
    (`PrimitiveComponent.SetCollisionEnabled` (`self.Capsule1`) "QueryAndPhysics")
    (else
      (`PrimitiveComponent.SetCollisionEnabled` (`self.Capsule`) "QueryAndPhysics"))))

(event `TurnOffAttackCollision`
  (if (`self.DarkChef`)
    (`PrimitiveComponent.SetCollisionEnabled` (`self.Capsule1`) "NoCollision")
    (else
      (`PrimitiveComponent.SetCollisionEnabled` (`self.Capsule`) "NoCollision"))))

(event `self.ReceivePointDamage`
  (params (Damage :type "Float (single-precision)") (DamageType :type "DamageType Object Reference") (HitLocation :type "Vector Structure") (HitNormal :type "Vector Structure") (HitComponent :type "PrimitiveComponent Object Reference") (BoneName :type Name) (ShotFromDirection :type "Vector Structure") (InstigatedBy :type "Controller Object Reference") (DamageCauser :type "Actor Object Reference") (HitInfo :type "HitResult Structure (by ref)"))
  (bind _mesh (`self.Mesh`))
  (bind _health (`self.Health`))
  (bind _charactermovement (`self.CharacterMovement`))
  (bind _chefhat (`self.ChefHat`))
  (bind _returnvalue (`SceneComponent.K2_GetComponentLocation` (`self.ChefHat`)))
  (bind _returnvalue_2 (`SceneComponent.K2_GetComponentLocation` (`self.ChefHat`)))
  (bind _returnvalue_3 (`SceneComponent.K2_GetComponentLocation` (`self.ChefHat`)))
  (if (== (`GameplayStatics.GetObjectClass` DamageType) "/Game/Blueprints/Damage/KnockBack_DamageType.KnockBack_DamageType_C")
    (`self.CannotMove`)
    (set `self.Stunned` true)
    (`KismetSystemLibrary.DelayUntilNextTick`)
    (set `CharacterMovementComponent.GroundFriction` 0.0 (`self.CharacterMovement`))
    (`self.LaunchCharacter` (* ShotFromDirection Damage 20000.0) true)
    (`|PlayMontage` (`self.Mesh`) "/Game/Animations/Baker/Stunned_mixamo_com_Montage.Stunned_mixamo_com_Montage"
      (:`OnBlendOut`
        (`|PlayMontage` (`self.Mesh`) "/Game/Animations/Baker/Getting_Up__8__mixamo_com_Montage.Getting_Up__8__mixamo_com_Montage"
          (:`OnBlendOut`
            (`self.CanMoveAgain`))
          (:`OnInterrupted`
            _)))
      (:`OnInterrupted`
        _))
    (set `self.Stunned` false)
    (`self.ChasePlayer`)
    (else
      (set `self.Health` (+ (* Damage -1.0) _health))
      (`|ExecutionSequence`
        (:`then_0`
          (`|ExecutionSequence`
            (:`then_0`
              (if (<= (`self.Health`) 0.0)
                (`|ExecutionSequence`
                  (:`then_0`
                    (`/Engine/EditorBlueprintResources/StandardMacros.DoOnce` false
                      (:`Completed`
                        (set `self.Dead` true)
                        (`|ExecutionSequence`
                          (:`then_0`
                            (`self.TurnOffAttackCollision`)
                            (`PrimitiveComponent.SetCollisionEnabled` _mesh "QueryAndPhysics")
                            (`PrimitiveComponent.SetSimulatePhysics` _mesh true)
                            (`PrimitiveComponent.AddRadialImpulse` (`self.Mesh`) HitLocation 3000.0 3000.0 "RIF_Constant" true)
                            (set `SkeletalMeshComponent.bPauseAnims` true (`self.Mesh`))
                            (`PrimitiveComponent.SetCollisionEnabled` (`self.CapsuleComponent`) "NoCollision")
                            (set `CharacterMovementComponent.GravityScale` 0.0 _charactermovement)
                            (`PrimitiveComponent.SetEnableGravity` (`self.CapsuleComponent`) false)
                            (`CharacterMovementComponent.SetMovementMode` _charactermovement "MOVE_Flying" 0)
                            (`PrimitiveComponent.SetCollisionEnabled` _chefhat "QueryAndPhysics")
                            (`SceneComponent.K2_DetachFromComponent` _chefhat "KeepWorld" "KeepWorld" "KeepWorld" true)
                            (`PrimitiveComponent.SetSimulatePhysics` _chefhat true)
                            (`ActorComponent.K2_DestroyComponent` (`self.Sphere`))
                            (`ActorComponent.K2_DestroyComponent` (`self.Sphere1`)))
                          (:`then_1`
                            (bind _asbp_third_person_character (cast `/Game/Blueprints/BP_ThirdPersonCharacter` (`GameplayStatics.GetPlayerCharacter` 0)))
                            (bind _hudwidget (`/Game/Blueprints/BP_ThirdPersonCharacter.HUDWidget` _asbp_third_person_character))
                            (if (== (`/Game/UI/HUD_WBP.CurrentBoss` _hudwidget) self)
                              (`/Game/UI/HUD_WBP.FadeOutBossHealth` _hudwidget)))
                          (:`then_2`
                            (if (`self.DarkChef`)
                              (`GameplayStatics.PlaySoundAtLocation` "/Game/SFX/DarkChefDeath_Cue.DarkChefDeath_Cue" (`self.K2_GetActorLocation`) (struct) 1.0 1.0 0.0 null null null null)
                              (if (`self.MiniBoss`)
                                (bind _asbp_third_person_character_2 (cast `/Game/Blueprints/BP_ThirdPersonCharacter` (`GameplayStatics.GetPlayerCharacter` 0)))
                                (bind _asmusic_controller_bp (cast `/Game/Blueprints/MusicController_BP` (`ChildActorComponent.ChildActor` (`/Game/Blueprints/BP_ThirdPersonCharacter.MusicController` _asbp_third_person_character_2))))
                                (`/Game/Blueprints/MusicController_BP.StopBossMusic` _asmusic_controller_bp))))))))
                  (:`then_1`
                    (`PrimitiveComponent.AddRadialImpulse` (`self.Mesh`) HitLocation 3000.0 3000.0 "RIF_Constant" true)))
                (else
                  (`self.Flinch`))))
            (:`then_1`
              (if (`self.DarkChef`)
                (if (<= _health (* (`self.DarkChefHealth`) 0.5))
                  (`/Engine/EditorBlueprintResources/StandardMacros.DoOnce` false
                    (:`Completed`
                      (set `self.Max Walk Speed` 900.0)
                      (set `self.Stunned` true :!label _label_7)
                      (`self.TurnOffAttackCollision`)
                      (`self.CannotMove`)
                      (if (`self.DarkChef`)
                        (set `self.HitReactToPlay` "/Game/Animations/Baker/Baker_Taunt_Anim_Montage.Baker_Taunt_Anim_Montage")
                        (else
                          (switch `int` (`KismetMathLibrary.RandomIntegerInRange` 0 2)
                            (:`Default`
                              (set `self.HitReactToPlay` "/Game/Animations/Baker/Standing_React_Large_From_Left__2__mixamo_com_Montage.Standing_React_Large_From_Left__2__mixamo_com_Montage" :!label _label_8))
                            (:`0`
                              (goto _label_8))
                            (:`1`
                              (set `self.HitReactToPlay` "/Game/Animations/Baker/Standing_React_Large_From_Right__2__mixamo_com_Montage.Standing_React_Large_From_Right__2__mixamo_com_Montage"))
                            (:`2`
                              (set `self.HitReactToPlay` "/Game/Animations/Baker/Standing_React_Large_Gut__2__mixamo_com_Montage.Standing_React_Large_Gut__2__mixamo_com_Montage")))))
                      (`|PlayMontage` (`self.Mesh`) (`self.HitReactToPlay`)
                        (:`OnBlendOut`
                          (set `self.Stunned` false)
                          (`self.CanMoveAgain`))
                        (:`OnNotifyBegin`
                          (`|ExecutionSequence`
                            (:`then_0`
                              (set `self.Raging` true)
                              (`SceneComponent.SetHiddenInGame` (`self.Sphere`) false false)
                              (`SceneComponent.SetHiddenInGame` (`self.Sphere1`) false false)
                              (`GameplayStatics.SpawnEmitterAtLocation` "/Game/VFX/Bonuses/P_Refraction.P_Refraction" _returnvalue_2 (struct) (5.0 5.0 5.0))
                              (`GameplayStatics.SpawnEmitterAtLocation` "/Game/VFX/Bonuses/P_Refraction.P_Refraction" _returnvalue_2 (struct) (5.0 5.0 5.0))
                              (`KismetSystemLibrary.Delay` 0.2)
                              (`GameplayStatics.SpawnEmitterAtLocation` "/Game/VFX/Bonuses/P_Refraction.P_Refraction" _returnvalue_3 (struct) (5.0 5.0 5.0))
                              (`GameplayStatics.SpawnEmitterAtLocation` "/Game/VFX/Bonuses/P_Refraction.P_Refraction" _returnvalue_3 (struct) (5.0 5.0 5.0))
                              (`KismetSystemLibrary.Delay` 0.2)
                              (`GameplayStatics.SpawnEmitterAtLocation` "/Game/VFX/Bonuses/P_Refraction.P_Refraction" _returnvalue (struct) (5.0 5.0 5.0))
                              (`GameplayStatics.SpawnEmitterAtLocation` "/Game/VFX/Bonuses/P_Refraction.P_Refraction" _returnvalue (struct) (5.0 5.0 5.0)))
                            (:`then_1`
                              (if (`self.DarkChef`)
                                (`GameplayStatics.PlaySoundAtLocation` "/Game/SFX/RoarDarkChef_Cue.RoarDarkChef_Cue" (`self.K2_GetActorLocation`) (struct) 1.0 1.0 0.0 null null null null)))))))))))))
        (:`then_1`
          (bind _asbp_third_person_character_3 (cast `/Game/Blueprints/BP_ThirdPersonCharacter` (`GameplayStatics.GetPlayerCharacter` 0)))
          (bind _hudwidget_2 (`/Game/Blueprints/BP_ThirdPersonCharacter.HUDWidget` _asbp_third_person_character_3))
          (`UserWidget.PlayAnimation` _hudwidget_2 (`/Game/UI/HUD_WBP.HitAnimTargetDot` _hudwidget_2) 0.0 1 "Forward" 1.0 false))
        (:`then_2`
          (if (not (`self.DarkChef`))
            (`GameplayStatics.PlaySoundAtLocation` "/Game/SFX/BakerHurt4_Cue.BakerHurt4_Cue" (`self.K2_GetActorLocation`) (struct) 1.0 1.0 0.0 null null null null)))))))

(event `Flinch`
  (if (not (`self.DarkChef`))
    (goto _label_7)))

(fn `UserConstructionScript`)