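; Boss enemy AI that sleeps in a frozen pose until hit or triggered, then roars and chases the player with a per-tick AIMoveTo loop.
; A detection capsule triggers random montage attacks whose notifies toggle the damage capsule, while a distant player triggers a cooldown-gated dash pursuit.
; At half health it staggers invulnerably, then rages with faster movement, combos and lightning AoE.
; On death it shrinks while spewing cake projectiles, then destroys itself.
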(event `self.ReceiveBeginPlay`
  (set `self.Max Walk Speed` (`CharacterMovementComponent.MaxWalkSpeed` (`self.CharacterMovement`)))
  (`self.CannotMove`)
  (`|PlayMontage` (`self.Mesh`) "/Game/Animations/Boss/BaseAnims/T_poseIdleMimicPose_Montage.T_poseIdleMimicPose_Montage" 0.0))

(event `WakeUp`
  (`/Engine/EditorBlueprintResources/StandardMacros.DoOnce` false
    (:`Completed`
      (`self.Roar`))))

(event `ContinueWakingUp`
  (`|PlayMontage` (`self.Mesh`) "/Game/Animations/Boss/Equip_Montage.Equip_Montage"
    (:`OnCompleted`
      _)
    (:`OnInterrupted`
      _))
  (set `self.Awake` true)
  (set `self.CannotBeDamaged` false)
  (set `self.Stunned` false)
  (`self.CanMoveAgain`)
  (set `self.Attacking` false)
  (`KismetSystemLibrary.DelayUntilNextTick`)
  (`self.ChasePlayer`))

(event `self.ReceiveAnyDamage`
  (params (Damage :type "Float (single-precision)") (DamageType :type "DamageType Object Reference") (InstigatedBy :type "Controller Object Reference") (DamageCauser :type "Actor Object Reference"))
  (if (== (`GameplayStatics.GetObjectClass` DamageType) "/Game/Blueprints/Damage/WakeUpEnemyAI_DamageType.WakeUpEnemyAI_DamageType_C")
    (`self.WakeUp`)))

(event `ChasePlayer`
  (bind _returnvalue (`self.K2_GetActorLocation` (`GameplayStatics.GetPlayerCharacter` 0)))
  (if (not (or (`self.Dead`) (`self.Stunned`)))
    (bind (_outhit _returnvalue_2) (`KismetSystemLibrary.SphereTraceSingle` _returnvalue (- _returnvalue (0.0 0.0 5000.0)) 35.0 "TraceTypeQuery1"))
    (if _returnvalue_2
      (set `self.PlayerLocation` (`.Location` (`GameplayStatics.BreakHitResult` _outhit)))
      (else
        (set `self.PlayerLocation` _returnvalue)))
    (if (`PrimitiveComponent.IsOverlappingActor` (`self.PlayerDetectionCapsule`) (`GameplayStatics.GetPlayerCharacter` 0))
      (set `self.OverlappingPlayer` true)
      (`self.AttackPlayer`))
    (`|AIMoveTo` self (`self.PlayerLocation`) null
      (:`then`
        _)
      (:`OnSuccess`
        _)
      (:`OnFail`
        _))
    (`KismetSystemLibrary.DelayUntilNextTick`)
    (`self.ChasePlayer`)))

(event `CannotMove`
  (set `self.CantMove` true)
  (set `CharacterMovementComponent.MaxWalkSpeed` 0.0 (`self.CharacterMovement`) :!label _label)
  (`KismetSystemLibrary.Delay` 0.01)
  (if (`self.CantMove`)
    (goto _label)))

(event `CanMoveAgain`
  (bind _charactermovement (`self.CharacterMovement`))
  (`KismetSystemLibrary.Delay` 0.01)
  (`KismetSystemLibrary.DelayUntilNextTick`)
  (`KismetSystemLibrary.DelayUntilNextTick`)
  (set `self.CantMove` false)
  (set `CharacterMovementComponent.MaxWalkSpeed` (`self.Max Walk Speed`) _charactermovement)
  (set `CharacterMovementComponent.GroundFriction` 0.0 _charactermovement))

(event `self.ReceiveTick`
  (params (DeltaSeconds :type "Float (single-precision)"))
  (if (`self.Awake`)
    (if (`self.Dead`)
      _
      (elif (>= (`KismetMathLibrary.VSize` (- (`self.K2_GetActorLocation`) (`self.K2_GetActorLocation` (`GameplayStatics.GetPlayerCharacter` 0)))) 1500.0)
        (if (not (`self.ForcedPursueOnCD`))
          (set `self.ForcedPursueOnCD` true)
          (`|ExecutionSequence`
            (:`then_0`
              (`self.ForcedPursue`))
            (:`then_1`
              (`KismetSystemLibrary.RetriggerableDelay` 5.0)
              (set `self.ForcedPursueOnCD` false))))))))

(event `self.PlayerDetectionCapsule.OnComponentBeginOverlap`
  (params (OverlappedComponent :type "PrimitiveComponent Object Reference") (OtherActor :type "Actor Object Reference") (OtherComp :type "PrimitiveComponent Object Reference") (OtherBodyIndex :type Integer) (bFromSweep :type Boolean) (SweepResult :type "HitResult Structure (by ref)"))
  (cast `/Game/Blueprints/BP_ThirdPersonCharacter` OtherActor)
  (set `self.OverlappingPlayer` true)
  (if (`self.Awake`)
    (if (not (`self.Dead`))
      (`self.AttackPlayer`)
      (if (== (`self.AttackMontageToPlay`) "/Game/Animations/Boss/PursuerAttack/PursueAttack_Montage.PursueAttack_Montage")
        (if (`self.Attacking`)
          (if (not (`self.Stunned`))
            (`self.ForceFinishPursue`)))))))

(event `self.PlayerDetectionCapsule.OnComponentEndOverlap`
  (params (OverlappedComponent :type "PrimitiveComponent Object Reference") (OtherActor :type "Actor Object Reference") (OtherComp :type "PrimitiveComponent Object Reference") (OtherBodyIndex :type Integer))
  (cast `/Game/Blueprints/BP_ThirdPersonCharacter` OtherActor)
  (set `self.OverlappingPlayer` false))

(event `ForcedPursue`
  (bind _charactermovement (`self.CharacterMovement`))
  (bind _returnvalue (+ (`SceneComponent.K2_GetComponentLocation` (`self.Mesh`)) (0.0 0.0 15.0)))
  (bind _asbp_third_person_character (cast `/Game/Blueprints/BP_ThirdPersonCharacter` (`GameplayStatics.GetPlayerCharacter` 0)))
  (if (`/Game/Blueprints/BP_ThirdPersonCharacter.PlayerDead` _asbp_third_person_character)
    (`|PlayMontage` (`self.Mesh`) "/Game/Animations/Boss/Hip_Hop_Dancing_mixamo_com_Montage.Hip_Hop_Dancing_mixamo_com_Montage" :!label _label_2
      (:`OnCompleted`
        (`|ExecutionSequence`
          (:`then_0`
            (goto _label_2)))))
    (elif (not (`self.Stunned`))
      (set `self.Attacking` true)
      (`self.CannotMove`)
      (set `self.AttackMontageToPlay` "/Game/Animations/Boss/PursuerAttack/PursueAttack_Montage.PursueAttack_Montage")
      (bind _notifyname (`|PlayMontage` (`self.Mesh`) (`self.AttackMontageToPlay`) :!label _label_3)
        (:`then`
          (if (== (`self.AttackMontageToPlay`) "/Game/Animations/Boss/AoE_Attack.AoE_Attack")
            (set `self.ChargingAttack` true)
            (`GameplayStatics.SpawnEmitterAtLocation` null (`self.K2_GetActorLocation`) :!label _label_4)
            (`KismetSystemLibrary.Delay` 0.2)
            (if (`self.ChargingAttack`)
              (goto _label_4))))
        (:`OnBlendOut`
          (set `self.Attacking` false)
          (`self.TurnOffAttackCollision`)
          (if (`self.OverlappingPlayer`)
            (`KismetSystemLibrary.DelayUntilNextTick`)
            (`self.AttackPlayer`)
            (else
              (`KismetSystemLibrary.DelayUntilNextTick`)
              (`self.CanMoveAgain`)
              (`self.ChasePlayer`))))
        (:`OnInterrupted`
          (`|ExecutionSequence`
            (:`then_1`
              (`self.TurnOffAttackCollision` :!label _label_5)
              (bind _returnvalue_2 (== _notifyname "Dash"))
              (if _returnvalue_2
                (`self.CannotMove`)
                (if (`self.Raging`)
                  (set `self.Max Walk Speed` 750.0)
                  (else
                    (set `self.Max Walk Speed` 400.0)))
                (set `CharacterMovementComponent.MaxAcceleration` 2048.0 _charactermovement)
                (`ActorComponent.Deactivate` (`self.FireBoots1`))
                (`ActorComponent.Deactivate` (`self.FireBoots`))))))
        (:`OnNotifyBegin`
          (`self.TurnOnAttackCollision`)
          (if (and (== _notifyname "Cast") (== (`self.AttackMontageToPlay`) "/Game/Animations/Boss/AoE_Attack.AoE_Attack"))
            ;[1 0.02496 0] Add AoE Attack Here
            (set `self.ChargingAttack` false)
            (`|SpawnActorFromClass` "/Game/Blueprints/Projectiles/EnemyLightningSpawner_BP.EnemyLightningSpawner_BP_C" (`KismetMathLibrary.MakeTransform` _returnvalue) "Undefined" "MultiplyWithRoot" self null)
            (`|SpawnActorFromClass` "/Game/Blueprints/Projectiles/EnemyLightningSpawner_BP.EnemyLightningSpawner_BP_C" (`KismetMathLibrary.MakeTransform` _returnvalue) "Undefined" "MultiplyWithRoot" self null)
            (`|SpawnActorFromClass` "/Game/Blueprints/Projectiles/EnemyLightningSpawner_BP.EnemyLightningSpawner_BP_C" (`KismetMathLibrary.MakeTransform` _returnvalue) "Undefined" "MultiplyWithRoot" self null)
            (elif _returnvalue_2
              (set `self.Max Walk Speed` 5000.0)
              (`self.CanMoveAgain`)
              (set `CharacterMovementComponent.MaxAcceleration` 99999.0 _charactermovement)
              (`ActorComponent.Activate` (`self.FireBoots`) true)
              (`ActorComponent.Activate` (`self.FireBoots1`) true))))
        (:`OnNotifyEnd`
          (goto _label_5))))))

(event `AttackPlayer`
  (bind _asbp_third_person_character (cast `/Game/Blueprints/BP_ThirdPersonCharacter` (`GameplayStatics.GetPlayerCharacter` 0)))
  (if (`/Game/Blueprints/BP_ThirdPersonCharacter.PlayerDead` _asbp_third_person_character)
    (goto _label_2)
    (elif (not (or (`self.Attacking`) (`self.Stunned`)))
      (set `self.Attacking` true)
      (`self.CannotMove`)
      (if (`self.Raging`)
        (switch `int` (`KismetMathLibrary.RandomIntegerInRange` 0 3)
          (:`Default`
            (switch `int` (`KismetMathLibrary.RandomIntegerInRange` 0 2) :!label _label_6
              (:`Default`
                _)
              (:`0`
                _)
              (:`1`
                (set `self.AttackMontageToPlay` "/Game/Animations/Boss/Upwards_Slash_Attack.Upwards_Slash_Attack")
                (goto _label_3))
              (:`2`
                (goto _label_3)))
            (set `self.AttackMontageToPlay` "/Game/Animations/Boss/DownSlash_Attack.DownSlash_Attack")
            (goto _label_3))
          (:`0`
            (set `self.AttackMontageToPlay` "/Game/Animations/Boss/4AttackCombo_Attack.4AttackCombo_Attack")
            (goto _label_3))
          (:`1`
            (set `self.AttackMontageToPlay` "/Game/Animations/Boss/AoE_Attack.AoE_Attack")
            (goto _label_3))
          (:`2`
            (goto _label_3))
          (:`3`
            (goto _label_6))
          (:`4`
            (`self.Roar`)))
        (else
          (goto _label_6))))))

(event `ForceFinishPursue`
  (set `self.AttackMontageToPlay` "/Game/Animations/Boss/PursuerAttack/PursuerAttack_BaseAnim_Montage.PursuerAttack_BaseAnim_Montage")
  (goto _label_3))

(event `self.Capsule1.OnComponentBeginOverlap`
  (params (OverlappedComponent :type "PrimitiveComponent Object Reference") (OtherActor :type "Actor Object Reference") (OtherComp :type "PrimitiveComponent Object Reference") (OtherBodyIndex :type Integer) (bFromSweep :type Boolean) (SweepResult :type "HitResult Structure (by ref)"))
  (bind _asbp_third_person_character (cast `/Game/Blueprints/BP_ThirdPersonCharacter` OtherActor))
  (if (`/Game/Blueprints/BP_ThirdPersonCharacter.PlayerDead` _asbp_third_person_character)
    (goto _label_2)
    (else
      (`GameplayStatics.ApplyPointDamage` _asbp_third_person_character (`self.Base Damage`) (`KismetMathLibrary.GetDirectionUnitVector` (`self.K2_GetActorLocation`) (`self.K2_GetActorLocation` _asbp_third_person_character)) SweepResult null self))))

(event `TurnOnAttackCollision`
  (`PrimitiveComponent.SetCollisionEnabled` (`self.Capsule1`) "QueryAndPhysics"))

(event `TurnOffAttackCollision`
  (`PrimitiveComponent.SetCollisionEnabled` (`self.Capsule1`) "NoCollision"))

(event `self.ReceivePointDamage`
  (params (Damage :type "Float (single-precision)") (DamageType :type "DamageType Object Reference") (HitLocation :type "Vector Structure") (HitNormal :type "Vector Structure") (HitComponent :type "PrimitiveComponent Object Reference") (BoneName :type Name) (ShotFromDirection :type "Vector Structure") (InstigatedBy :type "Controller Object Reference") (DamageCauser :type "Actor Object Reference") (HitInfo :type "HitResult Structure (by ref)"))
  (bind _mesh (`self.Mesh`))
  (bind _health (`self.Health`))
  (bind _charactermovement (`self.CharacterMovement`))
  (bind _cakestospawnondeath (`self.CakesToSpawnOnDeath`))
  (bind _mesh_2 (`self.Mesh`))
  (bind _returnvalue_location (`KismetMathLibrary.BreakTransform` (`SkinnedMeshComponent.GetBoneTransform` (`self.Mesh`) "Head" "RTS_World")))
  (bind _returnvalue_location_2 (`KismetMathLibrary.BreakTransform` (`SkinnedMeshComponent.GetBoneTransform` (`self.Mesh`) "Head" "RTS_World")))
  (bind _returnvalue_location_3 (`KismetMathLibrary.BreakTransform` (`SkinnedMeshComponent.GetBoneTransform` (`self.Mesh`) "Head" "RTS_World")))
  (bind _returnvalue (+ _returnvalue_location_3 (0.0 0.0 55.0)))
  (if (`self.Awake`)
    (if (not (`self.CannotBeDamaged`))
      (set `self.Health` (+ (* Damage -1.0) _health))
      (`|ExecutionSequence`
        (:`then_0`
          (`|ExecutionSequence`
            (:`then_0`
              (if (<= (`self.Health`) 0.0)
                (`|ExecutionSequence`
                  (:`then_0`
                    (`/Engine/EditorBlueprintResources/StandardMacros.DoOnce` false
                      (:`Completed`
                        (set `self.Dead` true)
                        (`self.CannotMove`)
                        (`|ExecutionSequence`
                          (:`then_0`
                            (`self.TurnOffAttackCollision`)
                            (set `self.Stunned` true)
                            (set `self.Attacking` true)
                            (`PrimitiveComponent.SetCollisionEnabled` (`self.CapsuleComponent`) "NoCollision")
                            (set `CharacterMovementComponent.GravityScale` 0.0 _charactermovement)
                            (`PrimitiveComponent.SetEnableGravity` (`self.CapsuleComponent`) false)
                            (`CharacterMovementComponent.SetMovementMode` _charactermovement "MOVE_Flying" 0)
                            (`|PlayMontage` (`self.Mesh`) "/Game/Animations/Boss/DeathAnim_Montage.DeathAnim_Montage"
                              (:`OnNotifyBegin`
                                (`|SpawnActorFromClass` "/Game/Blueprints/CakeProjectile_BP.CakeProjectile_BP_C" (`KismetMathLibrary.MakeTransform` _returnvalue (`KismetMathLibrary.Conv_VectorToRotator` (`KismetMathLibrary.RandomUnitVectorInConeInDegrees` (`self.GetActorUpVector`) 55.0))) "Undefined" "MultiplyWithRoot" null false null :!label _label_7)
                                (`GameplayStatics.SpawnEmitterAtLocation` "/Game/VFX/P_SquirtGun.P_SquirtGun" _returnvalue)
                                (`SceneComponent.SetRelativeScale3D` _mesh_2 (* (`SceneComponent.RelativeScale3D` _mesh_2) 0.98))
                                (`/Engine/EditorBlueprintResources/StandardMacros.DecrementInt` _cakestospawnondeath
                                  (:`  `
                                    (if (<= _cakestospawnondeath 0)
                                      (`self.K2_DestroyActor`)
                                      (else
                                        (`KismetSystemLibrary.Delay` 0.05)
                                        (goto _label_7))))))))
                          (:`then_1`
                            (`ActorComponent.Deactivate` (`self.FireBoots1`))
                            (`ActorComponent.Deactivate` (`self.FireBoots`)))))))
                  (:`then_1`
                    (`PrimitiveComponent.AddRadialImpulse` (`self.Mesh`) HitLocation 3000.0 3000.0 "RIF_Constant" true)))))
            (:`then_1`
              (if (<= _health (* (`self.MaxHealth`) 0.5))
                (`/Engine/EditorBlueprintResources/StandardMacros.DoOnce` false :!label _label_8
                  (:`Completed`
                    (`|ExecutionSequence`
                      (:`then_0`
                        (set `self.CannotBeDamaged` true)
                        (set `self.Max Walk Speed` 750.0)
                        (set `self.Stunned` true)
                        (`self.TurnOffAttackCollision`)
                        (`self.CannotMove`)
                        (set `self.HitReactToPlay` "/Game/Animations/Boss/BossStage1Over.BossStage1Over")
                        (`ActorComponent.Deactivate` (`self.FireBoots1`))
                        (`ActorComponent.Deactivate` (`self.FireBoots`))
                        (`|PlayMontage` _mesh (`self.HitReactToPlay`)
                          (:`OnBlendOut`
                            (`|PlayMontage` _mesh "/Game/Animations/Boss/BossGettingUp2ndStage.BossGettingUp2ndStage"
                              (:`OnBlendOut`
                                (`|PlayMontage` _mesh "/Game/Animations/Boss/BattlecryMontage.BattlecryMontage" :!label _label_9
                                  (:`OnBlendOut`
                                    (if (`self.Awake`)
                                      (set `self.CannotBeDamaged` false)
                                      (set `self.Stunned` false)
                                      (`self.CanMoveAgain`)
                                      (set `self.Attacking` false)
                                      (`KismetSystemLibrary.DelayUntilNextTick`)
                                      (`self.ChasePlayer`)
                                      (else
                                        (`self.ContinueWakingUp`))))
                                  (:`OnNotifyBegin`
                                    (if (`self.Awake`)
                                      (set `self.Raging` true))
                                    (`GameplayStatics.SpawnEmitterAtLocation` "/Game/VFX/Bonuses/P_Refraction.P_Refraction" _returnvalue_location (struct) (5.0 5.0 5.0))
                                    (`GameplayStatics.SpawnEmitterAtLocation` "/Game/VFX/Bonuses/P_Refraction.P_Refraction" _returnvalue_location (struct) (5.0 5.0 5.0))
                                    (`KismetSystemLibrary.Delay` 0.2)
                                    (`GameplayStatics.SpawnEmitterAtLocation` "/Game/VFX/Bonuses/P_Refraction.P_Refraction" _returnvalue_location (struct) (5.0 5.0 5.0))
                                    (`GameplayStatics.SpawnEmitterAtLocation` "/Game/VFX/Bonuses/P_Refraction.P_Refraction" _returnvalue_location (struct) (5.0 5.0 5.0))
                                    (`KismetSystemLibrary.Delay` 0.2)
                                    (`GameplayStatics.SpawnEmitterAtLocation` "/Game/VFX/Bonuses/P_Refraction.P_Refraction" _returnvalue_location (struct) (5.0 5.0 5.0))
                                    (`GameplayStatics.SpawnEmitterAtLocation` "/Game/VFX/Bonuses/P_Refraction.P_Refraction" _returnvalue_location (struct) (5.0 5.0 5.0))
                                    (`KismetSystemLibrary.Delay` 0.2)
                                    (`GameplayStatics.SpawnEmitterAtLocation` "/Game/VFX/Bonuses/P_Refraction.P_Refraction" _returnvalue_location (struct) (5.0 5.0 5.0))
                                    (`GameplayStatics.SpawnEmitterAtLocation` "/Game/VFX/Bonuses/P_Refraction.P_Refraction" _returnvalue_location (struct) (5.0 5.0 5.0))
                                    (`KismetSystemLibrary.Delay` 0.2)
                                    (`GameplayStatics.SpawnEmitterAtLocation` "/Game/VFX/Bonuses/P_Refraction.P_Refraction" _returnvalue_location (struct) (5.0 5.0 5.0))
                                    (`GameplayStatics.SpawnEmitterAtLocation` "/Game/VFX/Bonuses/P_Refraction.P_Refraction" _returnvalue_location (struct) (5.0 5.0 5.0))
                                    (`KismetSystemLibrary.Delay` 0.2)
                                    (`GameplayStatics.SpawnEmitterAtLocation` "/Game/VFX/Bonuses/P_Refraction.P_Refraction" _returnvalue_location_2 (struct) (5.0 5.0 5.0))
                                    (`GameplayStatics.SpawnEmitterAtLocation` "/Game/VFX/Bonuses/P_Refraction.P_Refraction" _returnvalue_location_2 (struct) (5.0 5.0 5.0))
                                    (`KismetSystemLibrary.Delay` 0.2)
                                    (`GameplayStatics.SpawnEmitterAtLocation` "/Game/VFX/Bonuses/P_Refraction.P_Refraction" _returnvalue_location_2 (struct) (5.0 5.0 5.0))
                                    (`GameplayStatics.SpawnEmitterAtLocation` "/Game/VFX/Bonuses/P_Refraction.P_Refraction" _returnvalue_location_2 (struct) (5.0 5.0 5.0))
                                    (`KismetSystemLibrary.Delay` 0.2)
                                    (`GameplayStatics.SpawnEmitterAtLocation` "/Game/VFX/Bonuses/P_Refraction.P_Refraction" _returnvalue_location_2 (struct) (5.0 5.0 5.0))
                                    (`GameplayStatics.SpawnEmitterAtLocation` "/Game/VFX/Bonuses/P_Refraction.P_Refraction" _returnvalue_location_2 (struct) (5.0 5.0 5.0))
                                    (`KismetSystemLibrary.Delay` 0.2)
                                    (`GameplayStatics.SpawnEmitterAtLocation` "/Game/VFX/Bonuses/P_Refraction.P_Refraction" _returnvalue_location_2 (struct) (5.0 5.0 5.0))
                                    (`GameplayStatics.SpawnEmitterAtLocation` "/Game/VFX/Bonuses/P_Refraction.P_Refraction" _returnvalue_location_2 (struct) (5.0 5.0 5.0)))))))))
                      (:`then_1`
                        (`KismetSystemLibrary.Delay` 0.2)
                        (`self.TurnOffAttackCollision` :!label _label_10))
                      (:`then_2`
                        (goto _label_10)))))))))
        (:`then_1`
          (bind _asbp_third_person_character (cast `/Game/Blueprints/BP_ThirdPersonCharacter` (`GameplayStatics.GetPlayerCharacter` 0)))
          (bind _hudwidget (`/Game/Blueprints/BP_ThirdPersonCharacter.HUDWidget` _asbp_third_person_character))
          (`UserWidget.PlayAnimation` _hudwidget (`/Game/UI/HUD_WBP.HitAnimTargetDot` _hudwidget) 0.0 1 "Forward" 1.0 false))))
    (else
      (`self.WakeUp`))))

(event `Roar`
  (goto _label_9))

(event `Flinch`
  ;[0.7521 0 1] unhooked for boss
  (goto _label_8))

(fn `UserConstructionScript`)