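; EventBox_AI_BP is a box-volume actor that wakes up the enemy AI inside it as a group.
; One tick after BeginPlay, it caches every actor overlapping its Box, with no class filter or later refresh.
; When it receives damage of type WakeUpEnemyAI_DamageType, it relays that same damage type to each cached actor, using the damage system as the wake-up signal.
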(event `self.ReceiveBeginPlay`
  (`KismetSystemLibrary.DelayUntilNextTick`)
  (set `self.ActorsToAwaken` (`PrimitiveComponent.GetOverlappingActors` (`self.Box`) null)))

(event `self.ReceiveAnyDamage`
  (params (Damage :type "Float (single-precision)") (DamageType :type "DamageType Object Reference") (InstigatedBy :type "Controller Object Reference") (DamageCauser :type "Actor Object Reference"))
  (if (== (`GameplayStatics.GetObjectClass` DamageType) "/Game/Blueprints/Damage/WakeUpEnemyAI_DamageType.WakeUpEnemyAI_DamageType_C")
    (for _array_element (`self.ActorsToAwaken`)
      (`GameplayStatics.ApplyDamage` _array_element 1.0 null self "/Game/Blueprints/Damage/WakeUpEnemyAI_DamageType.WakeUpEnemyAI_DamageType_C"))))

(fn `UserConstructionScript`)