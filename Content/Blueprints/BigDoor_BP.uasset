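; Interactable double door that the player opens, driven by damage types used as interaction messages.
; An interact hit snaps the player to a wizard mesh reference point, freezes them and starts a timeline swinging both leaves open, while a reverse-interact hit can reverse it.
; The overlap box registers the door as nearby interactable until opening progress disables it.
; ForceCloseDoor animates it shut; point damage snaps it open.
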(event `self.ReceiveAnyDamage`
  (params (Damage :type "Float (single-precision)") (DamageType :type "DamageType Object Reference") (InstigatedBy :type "Controller Object Reference") (DamageCauser :type "Actor Object Reference"))
  (bind _wizardskeletalmeshlocationref (`self.WizardSkeletalMeshLocationRef`))
  (if (== (`GameplayStatics.GetObjectClass` DamageType) "/Game/Blueprints/Damage/Interact_DamageType.Interact_DamageType_C")
    (bind _asbp_third_person_character (cast `/Game/Blueprints/BP_ThirdPersonCharacter` (`GameplayStatics.GetPlayerCharacter` 0)))
    (`self.K2_TeleportTo` _asbp_third_person_character (`SceneComponent.K2_GetComponentLocation` _wizardskeletalmeshlocationref) (`SceneComponent.K2_GetComponentRotation` _wizardskeletalmeshlocationref))
    (`/Game/Blueprints/BP_ThirdPersonCharacter.CannotMove` _asbp_third_person_character)
    (`self.OpenDoor`)
    (set `/Game/Blueprints/BP_ThirdPersonCharacter.ActivelyWorkingInteractible` self _asbp_third_person_character)
    (`KismetSystemLibrary.DelayUntilNextTick`)
    (bind _asbp_third_person_character_2 (cast `/Game/Blueprints/BP_ThirdPersonCharacter` (`GameplayStatics.GetPlayerCharacter` 0)))
    (`Character.LaunchCharacter` _asbp_third_person_character (0.0 0.0 0.0) true true)
    (`Character.LaunchCharacter` _asbp_third_person_character_2 (0.0 0.0 0.0) true true)
    (set `MovementComponent.Velocity` (0.0 0.0 0.0) (`Character.CharacterMovement` _asbp_third_person_character_2))
    (elif (== (`GameplayStatics.GetObjectClass` DamageType) "/Game/Blueprints/Damage/ReverseInteract_DamageType.ReverseInteract_DamageType_C")
      (`self.CancelDoorOpening`)
      (bind _asbp_third_person_character_3 (cast `/Game/Blueprints/BP_ThirdPersonCharacter` (`GameplayStatics.GetPlayerCharacter` 0)))
      (set `/Game/Blueprints/BP_ThirdPersonCharacter.ActivelyWorkingInteractible` null _asbp_third_person_character_3))))

(event `OpenDoor`
  (`|ExecutionSequence`
    (:`then_0`
      (bind (_direction _newtrack_0) (`Timeline|Timeline` :!via `PlayFromStart` :!label _label)
        (:`Update`
          (`SceneComponent.K2_SetRelativeRotation` (`self.BigDoorLeft`) (`KismetMathLibrary.RLerp` (struct) (`self.LeftDoorEndRotation`) _newtrack_0) false false)
          (`SceneComponent.K2_SetRelativeRotation` (`self.BigDoorRight`) (`KismetMathLibrary.RLerp` (struct) (`self.RightDoorEndRotation`) _newtrack_0) false false)
          (if (>= _newtrack_0 0.2)
            (set `self.CannotCancel` false)
            (`PrimitiveComponent.SetCollisionEnabled` (`self.Box`) "NoCollision")
            (bind _asbp_third_person_character (cast `/Game/Blueprints/BP_ThirdPersonCharacter` (`GameplayStatics.GetPlayerCharacter` 0)))
            (if (== (`/Game/Blueprints/BP_ThirdPersonCharacter.ActivelyWorkingInteractible` _asbp_third_person_character) self)
              (set `/Game/Blueprints/BP_ThirdPersonCharacter.ActivelyWorkingInteractible` null _asbp_third_person_character)
              (elif (== (`/Game/Blueprints/BP_ThirdPersonCharacter.NearbyInteractibleActor` _asbp_third_person_character) self)
                (set `/Game/Blueprints/BP_ThirdPersonCharacter.NearbyInteractibleActor` null _asbp_third_person_character)))))))))

(event `CancelDoorOpening`
  (if (not (`self.CannotCancel`))
    (goto _label :!via `Reverse`)))

(event `ForceCloseDoor`
  (bind (_direction _newtrack_0) (`Timeline|Timeline_0` :!via `PlayFromStart`)
    (:`Update`
      (`SceneComponent.K2_SetRelativeRotation` (`self.BigDoorLeft`) (`KismetMathLibrary.RLerp` (`self.LeftDoorEndRotation`) (struct) _newtrack_0) false false)
      (`SceneComponent.K2_SetRelativeRotation` (`self.BigDoorRight`) (`KismetMathLibrary.RLerp` (`self.RightDoorEndRotation`) (struct) _newtrack_0) false false))))

(event `self.Box.OnComponentBeginOverlap`
  (params (OverlappedComponent :type "PrimitiveComponent Object Reference") (OtherActor :type "Actor Object Reference") (OtherComp :type "PrimitiveComponent Object Reference") (OtherBodyIndex :type Integer) (bFromSweep :type Boolean) (SweepResult :type "HitResult Structure (by ref)"))
  (bind _asbp_third_person_character (cast `/Game/Blueprints/BP_ThirdPersonCharacter` OtherActor))
  (set `/Game/Blueprints/BP_ThirdPersonCharacter.NearbyInteractibleActor` self _asbp_third_person_character))

(event `self.Box.OnComponentEndOverlap`
  (params (OverlappedComponent :type "PrimitiveComponent Object Reference") (OtherActor :type "Actor Object Reference") (OtherComp :type "PrimitiveComponent Object Reference") (OtherBodyIndex :type Integer))
  (bind _asbp_third_person_character (cast `/Game/Blueprints/BP_ThirdPersonCharacter` OtherActor))
  (if (== (`/Game/Blueprints/BP_ThirdPersonCharacter.NearbyInteractibleActor` _asbp_third_person_character) self)
    (set `/Game/Blueprints/BP_ThirdPersonCharacter.NearbyInteractibleActor` null _asbp_third_person_character)))

(event `self.ReceivePointDamage`
  (params (Damage :type "Float (single-precision)") (DamageType :type "DamageType Object Reference") (HitLocation :type "Vector Structure") (HitNormal :type "Vector Structure") (HitComponent :type "PrimitiveComponent Object Reference") (BoneName :type Name) (ShotFromDirection :type "Vector Structure") (InstigatedBy :type "Controller Object Reference") (DamageCauser :type "Actor Object Reference") (HitInfo :type "HitResult Structure (by ref)"))
  (`SceneComponent.K2_SetRelativeRotation` (`self.BigDoorLeft`) (`self.LeftDoorEndRotation`) false false)
  (`SceneComponent.K2_SetRelativeRotation` (`self.BigDoorRight`) (`self.RightDoorEndRotation`) false false))

(fn `UserConstructionScript`)