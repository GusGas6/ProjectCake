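; Cake pickup that the third-person character collects by touching it.
; On BeginPlay it picks one of five frosting materials at random and bobs the cake up and down in an endless eased MoveComponentTo loop with slightly randomized timing.
; When a living player overlaps the sphere, it signals the pickup through ApplyDamage with a custom AdjustCake damage type, then destroys itself.
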(event `self.ReceiveBeginPlay`
  (bind _cakeshape (`self.CakeShape`))
  (bind _cakeshape_2 (`self.CakeShape`))
  (bind _startlocationorb (`self.StartLocationOrb`))
  (bind _hovertimer (`self.HoverTimer`))
  (set `self.HoverTimer` (`KismetMathLibrary.RandomFloatInRange` 0.9 1.1))
  (`|ExecutionSequence`
    (:`then_0`
      (set `self.StartLocationOrb` (`SceneComponent.RelativeLocation` _cakeshape))
      (set `self.StartRotationOrb` (`SceneComponent.RelativeRotation` _cakeshape))
      (`KismetSystemLibrary.MoveComponentTo` _cakeshape (+ _startlocationorb (0.0 0.0 40.0)) (`KismetMathLibrary.MakeRotator` 0.0) true true _hovertimer :!label _label)
      (`KismetSystemLibrary.MoveComponentTo` _cakeshape _startlocationorb (`KismetMathLibrary.MakeRotator` 0.0) true true _hovertimer)
      (goto _label))
    (:`then_1`
      (switch `int` (`KismetMathLibrary.RandomIntegerInRange` 0 4)
        (:`Default`
          (`PrimitiveComponent.SetMaterial` _cakeshape_2 0 "/Game/Materials/Frosting_mat1.Frosting_mat1" :!label _label_2))
        (:`0`
          (goto _label_2))
        (:`1`
          (`PrimitiveComponent.SetMaterial` _cakeshape_2 0 "/Game/Materials/RandomFrosting_Mat1.RandomFrosting_Mat1"))
        (:`2`
          (`PrimitiveComponent.SetMaterial` _cakeshape_2 0 "/Game/Materials/RandomFrosting_Mat2.RandomFrosting_Mat2"))
        (:`3`
          (`PrimitiveComponent.SetMaterial` _cakeshape_2 0 "/Game/Materials/RandomFrosting_Mat3.RandomFrosting_Mat3"))
        (:`4`
          (`PrimitiveComponent.SetMaterial` _cakeshape_2 0 "/Game/Materials/RandomFrosting_Mat4.RandomFrosting_Mat4"))))))

(event `self.Sphere.OnComponentBeginOverlap`
  (params (OverlappedComponent :type "PrimitiveComponent Object Reference") (OtherActor :type "Actor Object Reference") (OtherComp :type "PrimitiveComponent Object Reference") (OtherBodyIndex :type Integer) (bFromSweep :type Boolean) (SweepResult :type "HitResult Structure (by ref)"))
  (bind _asbp_third_person_character (cast `/Game/Blueprints/BP_ThirdPersonCharacter` OtherActor))
  (if (not (`/Game/Blueprints/BP_ThirdPersonCharacter.PlayerDead` _asbp_third_person_character))
    (`GameplayStatics.ApplyDamage` OtherActor 1.0 null self "/Game/Blueprints/Damage/AdjustCake_DamageType.AdjustCake_DamageType_C")
    (`self.K2_DestroyActor`)))

(fn `UserConstructionScript`)