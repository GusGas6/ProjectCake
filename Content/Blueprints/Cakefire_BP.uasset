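; Cakefire is a bonfire-style checkpoint that the player lights to save a respawn point.
; An overlap sphere registers it as the player's nearby interactible while unlit.
; Custom damage types act as messages: interact snaps and freezes the player at its skeletal mesh, and light triggers candle flames, audio, particles and a HUD animation.
; Lighting also saves the transform and the player's cake amount to the game mode and clears the player's interaction references.
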(event `LightCakefire`
  (bind _skeletalmesh (`self.SkeletalMesh`))
  (set `self.CakefireLit` true)
  (`|ExecutionSequence`
    (:`then_0`
      (`SceneComponent.SetHiddenInGame` (`self.CandleFire7`) false false)
      (`SceneComponent.SetHiddenInGame` (`self.CandleFire8`) false false)
      (`SceneComponent.SetHiddenInGame` (`self.CandleFire2`) false false)
      (`SceneComponent.SetHiddenInGame` (`self.CandleFire3`) false false)
      (`SceneComponent.SetHiddenInGame` (`self.CandleFire4`) false false)
      (`SceneComponent.SetHiddenInGame` (`self.CandleFire5`) false false)
      (`SceneComponent.SetHiddenInGame` (`self.CandleFire6`) false false)
      (`SceneComponent.SetHiddenInGame` (`self.CandleFire`) false false)
      (`SceneComponent.SetHiddenInGame` (`self.CandleFire1`) false false)
      (`SceneComponent.SetHiddenInGame` (`self.PointLight`) false false)
      (`ActorComponent.Activate` (`self.Audio`) true)
      (bind _asbp_third_person_character (cast `/Game/Blueprints/BP_ThirdPersonCharacter` (`GameplayStatics.GetPlayerCharacter` 0)))
      (bind _asbp_third_person_game_mode (cast `/Game/ThirdPerson/Blueprints/BP_ThirdPersonGameMode` (`GameplayStatics.GetGameMode`)))
      (`/Game/ThirdPerson/Blueprints/BP_ThirdPersonGameMode.CakefireSaveRespawnLocation` _asbp_third_person_game_mode (`SceneComponent.K2_GetComponentLocation` _skeletalmesh) (`SceneComponent.K2_GetComponentRotation` _skeletalmesh) self (`/Game/Blueprints/BP_ThirdPersonCharacter.AmountOfCake` _asbp_third_person_character)))
    (:`then_1`
      (`KismetSystemLibrary.DelayUntilNextTick`)
      (bind _asbp_third_person_character_2 (cast `/Game/Blueprints/BP_ThirdPersonCharacter` (`GameplayStatics.GetPlayerCharacter` 0)))
      (set `/Game/Blueprints/BP_ThirdPersonCharacter.NearbyInteractibleActor` null _asbp_third_person_character_2)
      (set `/Game/Blueprints/BP_ThirdPersonCharacter.ActivelyWorkingInteractible` null _asbp_third_person_character_2))))

(event `self.ReceiveAnyDamage`
  (params (Damage :type "Float (single-precision)") (DamageType :type "DamageType Object Reference") (InstigatedBy :type "Controller Object Reference") (DamageCauser :type "Actor Object Reference"))
  (bind _skeletalmesh (`self.SkeletalMesh`))
  (if (`self.CakefireLit`)
    _
    (elif (== (`GameplayStatics.GetObjectClass` DamageType) "/Game/Blueprints/Damage/Interact_DamageType.Interact_DamageType_C")
      (bind _asbp_third_person_character (cast `/Game/Blueprints/BP_ThirdPersonCharacter` (`GameplayStatics.GetPlayerCharacter` 0)))
      (`self.K2_TeleportTo` _asbp_third_person_character (`SceneComponent.K2_GetComponentLocation` _skeletalmesh) (`SceneComponent.K2_GetComponentRotation` _skeletalmesh))
      (`/Game/Blueprints/BP_ThirdPersonCharacter.CannotMove` _asbp_third_person_character)
      (set `/Game/Blueprints/BP_ThirdPersonCharacter.ActivelyWorkingInteractible` self _asbp_third_person_character)
      (`KismetSystemLibrary.DelayUntilNextTick`)
      (bind _asbp_third_person_character_2 (cast `/Game/Blueprints/BP_ThirdPersonCharacter` (`GameplayStatics.GetPlayerCharacter` 0)))
      (`Character.LaunchCharacter` _asbp_third_person_character (0.0 0.0 0.0) true true)
      (`Character.LaunchCharacter` _asbp_third_person_character_2 (0.0 0.0 0.0) true true)
      (set `MovementComponent.Velocity` (0.0 0.0 0.0) (`Character.CharacterMovement` _asbp_third_person_character_2))
      (elif (== (`GameplayStatics.GetObjectClass` DamageType) "/Game/Blueprints/Damage/LightCakefire_DamageType.LightCakefire_DamageType_C")
        (`self.LightCakefire`)
        (`ActorComponent.Activate` (`self.ParticleSystem`) true)
        (bind _asbp_third_person_character_3 (cast `/Game/Blueprints/BP_ThirdPersonCharacter` (`GameplayStatics.GetPlayerCharacter` 0)))
        (bind _hudwidget (`/Game/Blueprints/BP_ThirdPersonCharacter.HUDWidget` _asbp_third_person_character_3))
        (`UserWidget.PlayAnimation` _hudwidget (`/Game/UI/HUD_WBP.CakefireLit` _hudwidget) 0.0 1 "Forward" 1.0 false)
        (`GameplayStatics.PlaySound2D` "/Game/SFX/LightBonfire1_Cue.LightBonfire1_Cue" 1.0 1.0 0.0 null null)))))

(event `self.Sphere.OnComponentBeginOverlap`
  (params (OverlappedComponent :type "PrimitiveComponent Object Reference") (OtherActor :type "Actor Object Reference") (OtherComp :type "PrimitiveComponent Object Reference") (OtherBodyIndex :type Integer) (bFromSweep :type Boolean) (SweepResult :type "HitResult Structure (by ref)"))
  (if (not (`self.CakefireLit`))
    (bind _asbp_third_person_character (cast `/Game/Blueprints/BP_ThirdPersonCharacter` OtherActor))
    (set `/Game/Blueprints/BP_ThirdPersonCharacter.NearbyInteractibleActor` self _asbp_third_person_character)))

(event `self.Sphere.OnComponentEndOverlap`
  (params (OverlappedComponent :type "PrimitiveComponent Object Reference") (OtherActor :type "Actor Object Reference") (OtherComp :type "PrimitiveComponent Object Reference") (OtherBodyIndex :type Integer))
  (bind _asbp_third_person_character (cast `/Game/Blueprints/BP_ThirdPersonCharacter` OtherActor))
  (if (== (`/Game/Blueprints/BP_ThirdPersonCharacter.NearbyInteractibleActor` _asbp_third_person_character) self)
    (set `/Game/Blueprints/BP_ThirdPersonCharacter.NearbyInteractibleActor` null _asbp_third_person_character)))

(fn `UserConstructionScript`)