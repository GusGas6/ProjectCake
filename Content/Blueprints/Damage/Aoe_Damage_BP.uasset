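; One-shot area-of-effect damage actor that sizes its sphere to AoERadius at BeginPlay and can ignore the player through a custom collision channel.
; On overlap it applies point damage directed away from its center and adds a velocity-change radial impulse to the sweep result's hit component.
; The first overlap schedules destruction for the next tick, or shows the debug sphere half a second longer with collision disabled.
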(event `self.ReceiveBeginPlay`
  (`|ExecutionSequence`
    (:`then_0`
      (if (`self.IgnorePlayer`)
        (`PrimitiveComponent.SetCollisionResponseToChannel` (`self.Sphere`) "ECC_GameTraceChannel1" "ECR_Ignore")))
    (:`then_1`
      (`SphereComponent.SetSphereRadius` (`self.Sphere`) (`self.AoERadius`) true)
      (if (`self.ShowDebugSphere`)
        (`SceneComponent.SetHiddenInGame` (`self.Sphere`) false false)))))

(event `self.Sphere.OnComponentBeginOverlap`
  (params (OverlappedComponent :type "PrimitiveComponent Object Reference") (OtherActor :type "Actor Object Reference") (OtherComp :type "PrimitiveComponent Object Reference") (OtherBodyIndex :type Integer) (bFromSweep :type Boolean) (SweepResult :type "HitResult Structure (by ref)"))
  (`GameplayStatics.ApplyPointDamage` OtherActor (`self.Base Damage`) (`KismetMathLibrary.GetDirectionUnitVector` (`self.K2_GetActorLocation`) (`self.K2_GetActorLocation` OtherActor)) SweepResult null self (`self.Damage Type Class`))
  (`PrimitiveComponent.AddRadialImpulse` (`.HitComponent` (`GameplayStatics.BreakHitResult` SweepResult)) (`self.K2_GetActorLocation`) (`self.ImpulseRadius`) (`self.ImpulseStrength`) "RIF_Constant" true)
  (if (`self.ShowDebugSphere`)
    (`KismetSystemLibrary.DelayUntilNextTick`)
    (`PrimitiveComponent.SetCollisionEnabled` (`self.Sphere`) "NoCollision")
    (`KismetSystemLibrary.Delay` 0.5)
    (else
      (`KismetSystemLibrary.DelayUntilNextTick`)))
  (`self.K2_DestroyActor`))

(fn `UserConstructionScript`)