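; A fake wall that opens like a secret door the first time it takes point damage.
; The hit scales up a Plane, plays the initial push audio and slides FakeWallMover back, then after a short pause lowers it with loop audio.
; During the descent, six chained timelines nudge FakeWallShaker sideways with rising then falling amplitude, layering a rumble over the main motion.
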(event `self.ReceiveBeginPlay`)

(event `self.ReceivePointDamage`
  (params (Damage :type "Float (single-precision)") (DamageType :type "DamageType Object Reference") (HitLocation :type "Vector Structure") (HitNormal :type "Vector Structure") (HitComponent :type "PrimitiveComponent Object Reference") (BoneName :type Name) (ShotFromDirection :type "Vector Structure") (InstigatedBy :type "Controller Object Reference") (DamageCauser :type "Actor Object Reference") (HitInfo :type "HitResult Structure (by ref)"))
  (`/Engine/EditorBlueprintResources/StandardMacros.DoOnce` false
    (:`Completed`
      (`|ExecutionSequence`
        (:`then_0`
          (bind (_direction _newtrack_0) (`Timeline|Timeline_4` :!via `PlayFromStart`)
            (:`Update`
              (`SceneComponent.SetRelativeScale3D` (`self.Plane`) (`KismetMathLibrary.VLerp` (0.0 0.0 0.0) (3.148547 3.148547 1.0) _newtrack_0)))))
        (:`then_1`
          (bind (_direction_2 _newtrack_0_2) (`Timeline|MoveBackTL` :!via `PlayFromStart`)
            (:`Update`
              (`SceneComponent.K2_SetRelativeLocation` (`self.FakeWallMover`) (`KismetMathLibrary.VLerp` (0.0 0.0 0.0) (-30.0 0.0 0.0) _newtrack_0_2) false false))
            (:`Finished`
              (`KismetSystemLibrary.Delay` 0.5)
              (`|ExecutionSequence`
                (:`then_0`
                  (bind (_direction_3 _newtrack_0_3) (`Timeline|MoveDownTL` :!via `PlayFromStart`)
                    (:`Update`
                      (`SceneComponent.K2_SetRelativeLocation` (`self.FakeWallMover`) (`KismetMathLibrary.VLerp` (-30.0 0.0 0.0) (-30.0 0.0 -960.0) _newtrack_0_3) false false))))
                (:`then_1`
                  (bind (_direction_4 _newtrack_0_4) (`Timeline|Timeline_2` :!via `PlayFromStart`)
                    (:`Update`
                      (`SceneComponent.K2_SetRelativeLocation` (`self.FakeWallShaker`) (`KismetMathLibrary.VLerp` (0.0 0.0 0.0) (0.0 1.0 0.0) _newtrack_0_4) false false))
                    (:`Finished`
                      (bind (_direction_5 _newtrack_0_5) (`Timeline|Timeline_3` :!via `PlayFromStart`)
                        (:`Update`
                          (`SceneComponent.K2_SetRelativeLocation` (`self.FakeWallShaker`) (`KismetMathLibrary.VLerp` (0.0 0.0 0.0) (0.0 2.5 0.0) _newtrack_0_5) false false))
                        (:`Finished`
                          (bind (_direction_6 _newtrack_0_6) (`Timeline|ShakeTL` :!via `PlayFromStart`)
                            (:`Update`
                              (`SceneComponent.K2_SetRelativeLocation` (`self.FakeWallShaker`) (`KismetMathLibrary.VLerp` (0.0 0.0 0.0) (0.0 5.0 0.0) _newtrack_0_6) false false))
                            (:`Finished`
                              (bind (_direction_7 _newtrack_0_7) (`Timeline|Timeline` :!via `PlayFromStart`)
                                (:`Update`
                                  (`SceneComponent.K2_SetRelativeLocation` (`self.FakeWallShaker`) (`KismetMathLibrary.VLerp` (0.0 0.0 0.0) (0.0 3.0 0.0) _newtrack_0_7) false false))
                                (:`Finished`
                                  (bind (_direction_8 _newtrack_0_8) (`Timeline|Timeline_0` :!via `PlayFromStart`)
                                    (:`Update`
                                      (`SceneComponent.K2_SetRelativeLocation` (`self.FakeWallShaker`) (`KismetMathLibrary.VLerp` (0.0 0.0 0.0) (0.0 2.0 0.0) _newtrack_0_8) false false))
                                    (:`Finished`
                                      (bind (_direction_9 _newtrack_0_9) (`Timeline|Timeline_1` :!via `PlayFromStart`)
                                        (:`Update`
                                          (`SceneComponent.K2_SetRelativeLocation` (`self.FakeWallShaker`) (`KismetMathLibrary.VLerp` (0.0 0.0 0.0) (0.0 1.0 0.0) _newtrack_0_9) false false))))))))))))))
                (:`then_2`
                  (`ActorComponent.Activate` (`self.PushLoopAudio`) true))))))
        (:`then_2`
          (`ActorComponent.Activate` (`self.InitialPushAudio`) true))))))

(fn `UserConstructionScript`)