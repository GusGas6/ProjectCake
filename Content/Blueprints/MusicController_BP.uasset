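; Music controller Blueprint that switches between the background soundtrack and two boss soundtracks.
; Background music fades in on BeginPlay, and the Tier 1 boss event fades it out before fading in the boss track.
; The Tier 2 event starts the second boss track without a fade.
; Stop events fade out each boss track, then deactivate it after a matching delay, and do not restart the background music.
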(event `self.ReceiveBeginPlay`
  (bind _backgroundsoundtrack (`self.BackgroundSoundtrack`))
  (`ActorComponent.Activate` _backgroundsoundtrack true)
  (`AudioComponent.FadeIn` _backgroundsoundtrack 5.0 1.0 0.0 "Linear"))

(event `Tier1BossMusic`
  (bind _backgroundsoundtrack (`self.BackgroundSoundtrack`))
  (bind _bosssoundtrack (`self.BossSoundtrack`))
  (`AudioComponent.FadeOut` _backgroundsoundtrack 2.0 0.0 "Linear")
  (`KismetSystemLibrary.Delay` 2.0)
  (`ActorComponent.Deactivate` _backgroundsoundtrack)
  (`AudioComponent.FadeIn` _bosssoundtrack 3.0 1.0 0.0 "Linear")
  (`ActorComponent.Activate` _bosssoundtrack true))

(event `StopBossMusic`
  (bind _bosssoundtrack (`self.BossSoundtrack`))
  (`AudioComponent.FadeOut` _bosssoundtrack 5.0 0.0 "Linear")
  (`KismetSystemLibrary.Delay` 5.0)
  (`ActorComponent.Deactivate` _bosssoundtrack))

(event `Tier2BossMusic`
  (`ActorComponent.Activate` (`self.BossSecondSoundtrack`) true))

(event `StopFinalBossMusic`
  (bind _bosssecondsoundtrack (`self.BossSecondSoundtrack`))
  (`AudioComponent.FadeOut` _bosssecondsoundtrack 5.0 0.0 "Linear")
  (`KismetSystemLibrary.Delay` 5.0)
  (`ActorComponent.Deactivate` _bosssecondsoundtrack))

(fn `UserConstructionScript`)