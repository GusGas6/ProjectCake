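; Crystal orb that hovers until an actor enters its sphere, then fires a MagicMissile_BP toward that actor and destroys itself.
; BeginPlay loops two eased MoveComponentTo calls with randomized durations to bob the mesh, and enables sphere collision after a short delay.
; Overlap waits a small random delay, then spawns the missile at the mesh, aimed at the stored actor if still valid.
; An unconnected debug line trace remains in the graph.
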(event `self.ReceiveBeginPlay`
  (bind _orbmesh (`self.OrbMesh`))
  (bind _startlocationorb (`self.StartLocationOrb`))
  (bind _hovertimer (`self.HoverTimer`))
  (bind _returnvalue (`KismetMathLibrary.RandomFloatInRange` _hovertimer (* _hovertimer (`KismetMathLibrary.RandomFloatInRange` 1.0 2.0))))
  (`|ExecutionSequence`
    (:`then_0`
      (set `self.StartLocationOrb` (`SceneComponent.RelativeLocation` _orbmesh))
      (set `self.StartRotationOrb` (`SceneComponent.RelativeRotation` _orbmesh))
      (`KismetSystemLibrary.MoveComponentTo` _orbmesh (+ _startlocationorb (0.0 0.0 5.0)) (`KismetMathLibrary.MakeRotator` 0.0) true true _returnvalue :!label _label)
      (`KismetSystemLibrary.MoveComponentTo` _orbmesh _startlocationorb (`KismetMathLibrary.MakeRotator` 0.0) true true _returnvalue)
      (goto _label))
    (:`then_1`
      (`KismetSystemLibrary.Delay` 0.5)
      (`PrimitiveComponent.SetCollisionEnabled` (`self.Sphere`) "QueryAndPhysics"))))

(event `self.Sphere.OnComponentBeginOverlap`
  (params (OverlappedComponent :type "PrimitiveComponent Object Reference") (OtherActor :type "Actor Object Reference") (OtherComp :type "PrimitiveComponent Object Reference") (OtherBodyIndex :type Integer) (bFromSweep :type Boolean) (SweepResult :type "HitResult Structure (by ref)"))
  (bind _overlappingactor (`self.OverlappingActor`))
  (bind _returnvalue (`SceneComponent.K2_GetComponentLocation` (`self.OrbMesh`)))
  (set `self.OverlappingActor` OtherActor)
  (`KismetSystemLibrary.Delay` (`KismetMathLibrary.RandomFloatInRange` 0.02 0.4))
  (`/Engine/EditorBlueprintResources/StandardMacros.IsValid` _overlappingactor
    (:`Is Valid`
      (`|SpawnActorFromClass` "/Game/Blueprints/Projectiles/MagicMissile_BP.MagicMissile_BP_C" (`KismetMathLibrary.MakeTransform` _returnvalue (`KismetMathLibrary.Conv_VectorToRotator` (`KismetMathLibrary.GetDirectionUnitVector` _returnvalue (`self.K2_GetActorLocation` _overlappingactor)))) "Undefined" "MultiplyWithRoot" null null)
      (`self.K2_DestroyActor`))))

(fn `UserConstructionScript`)