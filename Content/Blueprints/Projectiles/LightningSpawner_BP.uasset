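; LightningSpawner_BP is an actor that calls down a series of lightning strikes scattered around its location, then destroys itself.
; Each strike spawns a yellow zap Niagara effect at a random horizontal offset, plus an Aoe_Damage_BP that ignores the player and a thunder sound at that point.
; The strike event re-calls itself after a randomized delay scaled from DelayUntilLightningstrike until MaxLightningStrikes is reached.
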(event `self.ReceiveBeginPlay`
  (`self.LightningStrike`))

(event `LightningStrike`
  (bind (_returnvalue_x _returnvalue_y _returnvalue_z) (`KismetMathLibrary.BreakVector` (`self.K2_GetActorLocation`)))
  (bind _totalamountoflightningstrikes (`self.TotalAmountOfLightningStrikes`))
  (bind _delay_until_lightningstrike (`self.Delay Until Lightningstrike`))
  (bind _returnvalue (`NiagaraFunctionLibrary.SpawnSystemAtLocation` "/Game/Vefects/Zap_VFX/VFX/Zap/Particles/NS_Zap_03_Yellow.NS_Zap_03_Yellow" (`KismetMathLibrary.MakeVector` (+ _returnvalue_x (`KismetMathLibrary.RandomFloatInRange` -500.0 500.0)) (+ _returnvalue_y (`KismetMathLibrary.RandomFloatInRange` -500.0 500.0)) _returnvalue_z) (struct) (1.5 1.5 1.5)))
  (bind _returnvalue_2 (`SceneComponent.K2_GetComponentLocation` _returnvalue))
  (`|SpawnActorFromClass` "/Game/Blueprints/Damage/Aoe_Damage_BP.Aoe_Damage_BP_C" (`KismetMathLibrary.MakeTransform` _returnvalue_2) "Undefined" "MultiplyWithRoot" null (`self.Base Damage`) null 100.0 false 2000.0 2000.0 true null)
  (`GameplayStatics.SpawnSoundAtLocation` "/Game/SFX/LightningStrike1_Cue.LightningStrike1_Cue" _returnvalue_2 (struct) 1.0 1.0 0.0 null null)
  (`KismetSystemLibrary.Delay` (`KismetMathLibrary.RandomFloatInRange` (* _delay_until_lightningstrike 0.5) (+ _delay_until_lightningstrike _delay_until_lightningstrike)))
  (`/Engine/EditorBlueprintResources/StandardMacros.IncrementInt` _totalamountoflightningstrikes
    (:`  `
      (if (>= _totalamountoflightningstrikes (`self.MaxLightningStrikes`))
        (`self.K2_DestroyActor`)
        (else
          (`self.LightningStrike`))))))

(fn `UserConstructionScript`)