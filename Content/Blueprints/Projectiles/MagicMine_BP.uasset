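; MagicMine_BP is a magic mine that triggers once when something overlaps its sphere and deals area damage.
; Its rune scales through a timeline on spawn and bobs gently in an endless MoveComponentTo loop.
; The first overlap stops that timeline and plays a second scale timeline, which on finishing spawns Aoe_Damage_BP set to ignore the player, plays refraction and explosion effects, then destroys the mine.
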(event `self.ReceiveBeginPlay`
  (bind _rune (`self.Rune`))
  (bind _startlocationorb (`self.StartLocationOrb`))
  (`|ExecutionSequence`
    (:`then_0`
      (set `self.StartLocationOrb` (`SceneComponent.RelativeLocation` _rune))
      (set `self.StartRotationOrb` (`SceneComponent.RelativeRotation` _rune))
      (`KismetSystemLibrary.MoveComponentTo` _rune (+ _startlocationorb (0.0 0.0 2.0)) (`KismetMathLibrary.MakeRotator` 0.0) true true 2.0 :!label _label)
      (`KismetSystemLibrary.MoveComponentTo` _rune _startlocationorb (struct) true true 2.0)
      (goto _label))
    (:`then_1`
      (bind (_direction _newtrack_0) (`Timeline|Timeline` :!via `PlayFromStart` :!label _label_2)
        (:`Update`
          (`SceneComponent.SetWorldScale3D` (`self.Rune`) (`KismetMathLibrary.VLerp` (0.0 0.0 0.0) (1.0 1.0 1.0) _newtrack_0)))))))

(event `self.Sphere.OnComponentBeginOverlap`
  (params (OverlappedComponent :type "PrimitiveComponent Object Reference") (OtherActor :type "Actor Object Reference") (OtherComp :type "PrimitiveComponent Object Reference") (OtherBodyIndex :type Integer) (bFromSweep :type Boolean) (SweepResult :type "HitResult Structure (by ref)"))
  (bind _returnvalue (`self.K2_GetActorLocation`))
  (`/Engine/EditorBlueprintResources/StandardMacros.DoOnce` false
    (:`Completed`
      (`|ExecutionSequence`
        (:`then_0`
          (goto _label_2 :!via `Stop`))
        (:`then_1`
          (bind (_direction _newtrack_0) (`Timeline|Timeline_0` :!via `PlayFromStart`)
            (:`Update`
              (`SceneComponent.SetRelativeScale3D` (`self.Rune`) (`KismetMathLibrary.VLerp` (0.0 0.0 0.0) (1.0 1.0 1.0) _newtrack_0)))
            (:`Finished`
              (`|SpawnActorFromClass` "/Game/Blueprints/Damage/Aoe_Damage_BP.Aoe_Damage_BP_C" (`KismetMathLibrary.MakeTransform` _returnvalue) "Undefined" "MultiplyWithRoot" null 1.0 null 150.0 false 2000.0 2000.0 true null)
              (`GameplayStatics.SpawnEmitterAtLocation` "/Game/VFX/Bonuses/P_Refraction.P_Refraction" _returnvalue)
              (`GameplayStatics.SpawnEmitterAtLocation` "/Game/StarterContent/Particles/P_MineExplosion.P_MineExplosion" _returnvalue)
              (`KismetSystemLibrary.DelayUntilNextTick`)
              (`self.K2_DestroyActor`))))))))

(fn `UserConstructionScript`)