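; Spell pickup projectile that flies to the player and unlocks the spell set by its SpellEnum.
; On BeginPlay it passes the spell to its widget, sets the orb's material or mesh for certain spells, and starts audio.
; After a short delay it homes on the player's staff orb, with a timeline ramping homing acceleration.
; Overlapping the player unlocks the spell once, plays effects and sound, then destroys itself.
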(event `self.ReceiveBeginPlay`
  (bind _projectilemovement (`self.ProjectileMovement`))
  (bind _spellenum (`self.SpellEnum`))
  (bind _spellorb (`self.SpellOrb`))
  (`|ExecutionSequence`
    (:`then_0`
      (bind _asspell_pickup_wbp (cast `/Game/UI/SpellPickup_WBP` (`WidgetComponent.GetWidget` (`self.Widget`))))
      (`/Game/UI/SpellPickup_WBP.SetSpellPickUp` _asspell_pickup_wbp _spellenum))
    (:`then_1`
      (`KismetSystemLibrary.Delay` 0.5)
      (set `ProjectileMovementComponent.bIsHomingProjectile` true _projectilemovement)
      (bind _asbp_third_person_character (cast `/Game/Blueprints/BP_ThirdPersonCharacter` (`GameplayStatics.GetPlayerCharacter` 0)))
      (bind _aswizard_staff_bp (cast `/Game/Blueprints/WizardStaff_BP` (`ChildActorComponent.ChildActor` (`/Game/Blueprints/BP_ThirdPersonCharacter.StaffChildActor` _asbp_third_person_character))))
      (set `ProjectileMovementComponent.HomingTargetComponent` (`/Game/Blueprints/WizardStaff_BP.WizardOrb` _aswizard_staff_bp) _projectilemovement)
      (bind (_direction _newtrack_0) (`Timeline|Timeline` :!via `PlayFromStart`)
        (:`Update`
          (set `ProjectileMovementComponent.HomingAccelerationMagnitude` (`KismetMathLibrary.Lerp` 0.0 999999.0 _newtrack_0) _projectilemovement))))
    (:`then_2`
      (switch `/Game/Blueprints/Enums/Spell_Enum` _spellenum
        (:`NewEnumerator2`
          (`PrimitiveComponent.SetMaterial` _spellorb 0 "/Game/Materials/OrbLightning_Mat.OrbLightning_Mat"))
        (:`NewEnumerator3`
          (`PrimitiveComponent.SetMaterial` _spellorb 0 "/Game/Materials/Orb_Mine_Mat.Orb_Mine_Mat"))
        (:`NewEnumerator4`
          (`StaticMeshComponent.SetStaticMesh` _spellorb "/Game/Models/SM_MagicGreatsword_Pickup.SM_MagicGreatsword_Pickup")
          (`SceneComponent.SetWorldScale3D` _spellorb (0.5 0.5 0.5)))))
    (:`then_3`
      (`ActorComponent.Activate` (`self.Audio`) true))))

(event `self.Sphere.OnComponentBeginOverlap`
  (params (OverlappedComponent :type "PrimitiveComponent Object Reference") (OtherActor :type "Actor Object Reference") (OtherComp :type "PrimitiveComponent Object Reference") (OtherBodyIndex :type Integer) (bFromSweep :type Boolean) (SweepResult :type "HitResult Structure (by ref)"))
  (bind _asbp_third_person_character (cast `/Game/Blueprints/BP_ThirdPersonCharacter` OtherActor))
  (`/Engine/EditorBlueprintResources/StandardMacros.DoOnce` false
    (:`Completed`
      (`/Game/Blueprints/BP_ThirdPersonCharacter.UnlockSpell` _asbp_third_person_character (`self.SpellEnum`))
      (`GameplayStatics.SpawnEmitterAtLocation` "/Game/VFX/P_OrbSpellcast.P_OrbSpellcast" (`self.K2_GetActorLocation`))
      (`GameplayStatics.PlaySound2D` "/Game/SFX/New/SpellUnlock_Cue.SpellUnlock_Cue" 1.0 1.0 0.0 null null)
      (`self.K2_DestroyActor`))))

(fn `UserConstructionScript`)