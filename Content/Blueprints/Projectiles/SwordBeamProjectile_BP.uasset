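; Sword beam projectile that explodes on its first hit, spawning area damage that ignores the player.
; A DoOnce-guarded Hit applies a radial impulse to the struck component and spawns Aoe_Damage_BP with the projectile's damage and radius, plus Alert_AoE_BP.
; It plays explosion particles and sound, disables collision, hides the mesh and stops LeadUp, then destroys itself after a short delay.
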(event `self.ReceiveHit`
  (params (MyComp :type "PrimitiveComponent Object Reference") (Other :type "Actor Object Reference") (OtherComp :type "PrimitiveComponent Object Reference") (bSelfMoved :type Boolean) (HitLocation :type "Vector Structure") (HitNormal :type "Vector Structure") (NormalImpulse :type "Vector Structure") (Hit :type "HitResult Structure (by ref)"))
  (bind _returnvalue (`self.K2_GetActorLocation`))
  (bind _scale (`self.Scale`))
  (`/Engine/EditorBlueprintResources/StandardMacros.DoOnce` false
    (:`Completed`
      (`GameplayStatics.SpawnEmitterAtLocation` "/Game/VFX/P_OrbSpellcast.P_OrbSpellcast" HitLocation (struct) (0.5 0.5 0.5))
      (`PrimitiveComponent.AddRadialImpulse` OtherComp (`self.K2_GetActorLocation`) 4000.0 4000.0 "RIF_Constant" true)
      (`|SpawnActorFromClass` "/Game/Blueprints/Damage/Aoe_Damage_BP.Aoe_Damage_BP_C" (`KismetMathLibrary.MakeTransform` _returnvalue) "Undefined" "MultiplyWithRoot" null (`self.Base Damage`) null (`self.Ao ERadius`) false 2000.0 2000.0 true null)
      (`GameplayStatics.SpawnEmitterAtLocation` "/Game/VFX/Bonuses/P_Refraction.P_Refraction" _returnvalue (struct) _scale)
      (`GameplayStatics.SpawnEmitterAtLocation` "/Game/StarterContent/Particles/P_SwordExplosion.P_SwordExplosion" _returnvalue (struct) _scale)
      (`|SpawnActorFromClass` "/Game/Blueprints/AI/Alert_AoE_BP.Alert_AoE_BP_C" (`KismetMathLibrary.MakeTransform` HitLocation) "Undefined" "MultiplyWithRoot" null 500.0 null)
      (`PrimitiveComponent.SetCollisionEnabled` (`self.Box`) "NoCollision")
      (`SceneComponent.SetHiddenInGame` (`self.SwordBeamMesh`) true false)
      (`GameplayStatics.PlaySoundAtLocation` "/Game/SFX/New/SwordBeamImpact2_Cue.SwordBeamImpact2_Cue" (`self.K2_GetActorLocation`) (struct) 1.0 1.0 0.0 null null null null)
      (`ActorComponent.Deactivate` (`self.LeadUp`))
      (`KismetSystemLibrary.Delay` 0.5)
      (`self.K2_DestroyActor`))))

(fn `UserConstructionScript`)