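; Spell chest actor that opens once when the third-person character enters its sphere trigger and spawns a spell pickup.
; Opening plays a timeline that rotates the lid, spawns the projectile spell pickup with the chest's SpellEnum at a spawn point, and plays a sound.
; A Sword flag also hides the chest bottom mesh after spawning.
; SaveOpened sets the already-opened state by snapping the lid open and disabling the trigger's collision.
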(event `OpenChest`
  (`|ExecutionSequence`
    (:`then_0`
      (bind (_direction _newtrack_0) (`Timeline|Timeline` :!via `PlayFromStart`)
        (:`Update`
          (`SceneComponent.K2_SetRelativeRotation` (`self.ChestTopMesh`) (`KismetMathLibrary.RLerp` (struct) (struct :`Pitch` 190.0) _newtrack_0) false false))))
    (:`then_1`
      (`|SpawnActorFromClass` "/Game/Blueprints/Projectiles/SpellPickUp_Projectile_BP.SpellPickUp_Projectile_BP_C" (`KismetMathLibrary.MakeTransform` (`SceneComponent.K2_GetComponentLocation` (`self.SpellSpawnLocation`))) "Undefined" "MultiplyWithRoot" null (`self.Spell Enum`) null)
      (if (`self.Sword`)
        (`SceneComponent.SetVisibility` (`self.ChestBottomMesh`) false false)))
    (:`then_2`
      (`GameplayStatics.PlaySoundAtLocation` "/Game/SFX/New/ChestOpening1½_Cue.ChestOpening1½_Cue" (`self.K2_GetActorLocation`) (struct) 1.0 1.0 0.0 null null null null))))

(event `self.Sphere.OnComponentBeginOverlap`
  (params (OverlappedComponent :type "PrimitiveComponent Object Reference") (OtherActor :type "Actor Object Reference") (OtherComp :type "PrimitiveComponent Object Reference") (OtherBodyIndex :type Integer) (bFromSweep :type Boolean) (SweepResult :type "HitResult Structure (by ref)"))
  (cast `/Game/Blueprints/BP_ThirdPersonCharacter` OtherActor)
  (`/Engine/EditorBlueprintResources/StandardMacros.DoOnce` false
    (:`Completed`
      (`self.OpenChest`))))

(event `SaveOpened`
  (`SceneComponent.K2_SetRelativeRotation` (`self.ChestTopMesh`) (struct :`Pitch` 190.0) false false)
  (`PrimitiveComponent.SetCollisionEnabled` (`self.Sphere`) "NoCollision"))

(fn `UserConstructionScript`)