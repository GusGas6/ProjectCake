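; A floating story letter that shows the King's letter on the HUD while the player is nearby.
; On BeginPlay the mesh bobs up and down in an endless MoveComponentTo loop, while a self-calling delayed event keeps turning the actor's yaw toward the player.
; Sphere overlap with the third-person character shows the letter selected by TutorialEnum through its HUD widget, and leaving the sphere hides it.
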(event `RotateTowardsPlayer`
  (bind (_returnvalue_roll _returnvalue_pitch _returnvalue_yaw) (`KismetMathLibrary.BreakRotator` (`KismetMathLibrary.Conv_VectorToRotator` (`KismetMathLibrary.GetDirectionUnitVector` (`self.K2_GetActorLocation`) (`self.K2_GetActorLocation` (`GameplayStatics.GetPlayerCharacter` 0))))))
  (`self.K2_SetActorRotation` (`KismetMathLibrary.MakeRotator` 0.0 0.0 _returnvalue_yaw))
  (`KismetSystemLibrary.Delay` 0.01)
  (`self.RotateTowardsPlayer`))

(event `self.ReceiveBeginPlay`
  (bind _startlocationorb (`self.StartLocationOrb`))
  (bind _hovertimer (`self.HoverTimer`))
  (bind _staticmesh (`self.StaticMesh`))
  (`|ExecutionSequence`
    (:`then_0`
      (set `self.StartLocationOrb` (`SceneComponent.RelativeLocation` _staticmesh))
      (set `self.StartRotationOrb` (`SceneComponent.RelativeRotation` _staticmesh))
      (`KismetSystemLibrary.MoveComponentTo` _staticmesh (+ _startlocationorb (0.0 0.0 8.0)) (`KismetMathLibrary.MakeRotator` -40.0) true true _hovertimer :!label _label)
      (`KismetSystemLibrary.MoveComponentTo` _staticmesh _startlocationorb (`KismetMathLibrary.MakeRotator` -40.0) true true _hovertimer)
      (goto _label))
    (:`then_1`
      (`self.RotateTowardsPlayer`))))

(event `self.Sphere.OnComponentBeginOverlap`
  (params (OverlappedComponent :type "PrimitiveComponent Object Reference") (OtherActor :type "Actor Object Reference") (OtherComp :type "PrimitiveComponent Object Reference") (OtherBodyIndex :type Integer) (bFromSweep :type Boolean) (SweepResult :type "HitResult Structure (by ref)"))
  (bind _asbp_third_person_character (cast `/Game/Blueprints/BP_ThirdPersonCharacter` OtherActor))
  (`/Game/UI/HUD_WBP.ShowKingLetter` (`/Game/Blueprints/BP_ThirdPersonCharacter.HUDWidget` _asbp_third_person_character) (`self.Tutorial Enum`)))

(event `self.Sphere.OnComponentEndOverlap`
  (params (OverlappedComponent :type "PrimitiveComponent Object Reference") (OtherActor :type "Actor Object Reference") (OtherComp :type "PrimitiveComponent Object Reference") (OtherBodyIndex :type Integer))
  (bind _asbp_third_person_character (cast `/Game/Blueprints/BP_ThirdPersonCharacter` OtherActor))
  (`/Game/UI/HUD_WBP.HideKingLetter` (`/Game/Blueprints/BP_ThirdPersonCharacter.HUDWidget` _asbp_third_person_character)))

(fn `UserConstructionScript`)