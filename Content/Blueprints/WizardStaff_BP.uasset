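; Wizard staff Blueprint with a floating orb that bobs until the staff is ragdolled.
; BeginPlay caches the orb's relative transform, then loops two eased MoveComponentTo calls to raise and lower it slightly.
; RagdollStaff enables collision and physics on staff and orb, then immediately destroys the orb and its spellcast, hum and lightning components, leaving the staff simulating.
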(event `self.ReceiveBeginPlay`
  (bind _wizardorb (`self.WizardOrb`))
  (bind _startlocationorb (`self.StartLocationOrb`))
  (set `self.StartLocationOrb` (`SceneComponent.RelativeLocation` _wizardorb))
  (set `self.StartRotationOrb` (`SceneComponent.RelativeRotation` _wizardorb))
  (`KismetSystemLibrary.MoveComponentTo` _wizardorb (+ _startlocationorb (0.0 0.0 2.0)) (`KismetMathLibrary.MakeRotator` 0.0) true true 2.0 :!label _label)
  (`KismetSystemLibrary.MoveComponentTo` _wizardorb _startlocationorb (`KismetMathLibrary.MakeRotator` 0.0) true true 2.0)
  (goto _label))

(event `RagdollStaff`
  (bind _wizardstaff (`self.WizardStaff`))
  (`PrimitiveComponent.SetCollisionEnabled` _wizardstaff "QueryAndPhysics")
  (`PrimitiveComponent.SetCollisionEnabled` (`self.WizardOrb`) "QueryAndPhysics")
  (`PrimitiveComponent.SetSimulatePhysics` _wizardstaff true)
  (`PrimitiveComponent.SetSimulatePhysics` (`self.WizardOrb`) true)
  (`ActorComponent.K2_DestroyComponent` (`self.WizardOrb`))
  (`ActorComponent.K2_DestroyComponent` (`self.P_OrbSpellcast`))
  (`ActorComponent.K2_DestroyComponent` (`self.P_OrbHum`))
  (`ActorComponent.K2_DestroyComponent` (`self.LightningOrb`)))

(fn `UserConstructionScript`)